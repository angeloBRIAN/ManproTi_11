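; BP_2D_Vector is an interactive 2D vector arrow in the XZ plane that displays its length and angle.
; MoveVectorHead moves the head sphere to a finger position, sets the arrow's length from the actor origin, and reapplies its color.
; It derives the angle with Atan2 and rotates the arrow about negative Y.
; Tick writes length and angle to the text display, while Pickup and Drop are empty stubs.
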(event EventDrop)

(event EventTick
  (params (DeltaSeconds :type Float%20%28single-precision%29))
  (Rendering|Components|TextRender|SetText (Variables|Default|GetDisplay) (Utilities|Text|FormatText "{0}, {1}°" (Variables|/Script/Engine.ArrowComponent|GetArrowLength (Variables|Default|GetVectorArrow)) (Utilities|Text|ToText(Float) (Variables|Default|GetAngle%20XY) "HalfToEven" false true 1 324 0 1))))

(event EventPickup
  (params (Attach%20To :type Scene%20Component%20Object%20Reference)))

(fn ConstructionScript)

(fn MoveVectorHead
  (params (FingerPos :type Vector) (Vector%20Arrow :type Arrow%20Component%20Object%20Reference))
  (bind _returnvalue (Transformation|GetActorLocation))
  (bind (_x _y _z) (Math|Vector|BreakVector FingerPos))
  (bind (_x_2 _y_2 _z_2) (Math|Vector|BreakVector _returnvalue))
  (bind _returnvalue_2 (- FingerPos _returnvalue))
  (Variables|Default|SetVector%20Head%20Loc FingerPos)
  (Variables|/Script/Engine.ArrowComponent|SetArrowLength Vector%20Arrow (Math|Vector|Distance(Vector) (Math|Vector|MakeVector _x 0.0 _z) (Math|Vector|MakeVector _x_2 0.0 _z_2)))
  (Components|Arrow|SetArrowColor(LinearColor) Vector%20Arrow (Math|Conversions|ToLinearColor(Color) (Variables|/Script/Engine.ArrowComponent|GetArrowColor Vector%20Arrow)))
  (Transformation|SetWorldLocation (Variables|Default|GetSphere) FingerPos false false)
  (bind _output_get (Variables|Default|SetAngle%20XY (Class|KismetMathLibrary|DegAtan2 (.z _returnvalue_2) (.x _returnvalue_2))))
  (Transformation|SetWorldRotation Vector%20Arrow (Math|Vector|RotatorfromAxisandAngle "0.000000,-1.000000,0.000000" _output_get) false false))