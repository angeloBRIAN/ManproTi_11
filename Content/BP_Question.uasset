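; Vector math puzzle actor that poses an addition, subtraction, scalar multiplication or cross product question using spawned 3D arrow actors.
; On BeginPlay it spawns an answer vector and randomized question vectors, orients their arrows, and computes the expected result for its QuestionType.
; CheckAnswer compares the submitted endpoint by squared distance, or by direction dot product for cross products, and fires a one-time dispatcher when close enough.
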(event EventBeginPlay
  (bind _returnvalue (Transformation|GetActorLocation))
  (bind _returnvalue_2 (Transformation|GetActorRotation))
  (bind (_roll _pitch _yaw) (Math|Rotator|BreakRotator _returnvalue_2))
  (bind _returnvalue_3 (Game|SpawnActorfromClass "/Game/BP_VectorAnswer.BP_VectorAnswer_C" (Math|Transform|MakeTransform _returnvalue (Math|Rotator|MakeRotator _roll _pitch (- _yaw -9e+01)) "1.000000,1.000000,1.000000") "Undefined" 0 "(R=1.000000,G=0.000000,B=0.000000,A=1.000000)" 4e+01 0))
  (Variables|Default|SetAnswerVector _returnvalue_3)
  (bind _returnvalue_4 (Game|SpawnActorfromClass "/Game/BP_QuestionVector.BP_QuestionVector_C" (Math|Transform|MakeTransform _returnvalue _returnvalue_2 "1.000000,1.000000,1.000000") "Undefined" 0 "(R=0.000000,G=1.000000,B=0.000000,A=1.000000)" 0))
  (bind _output_get (Variables|Default|SetVector%201 _returnvalue_4))
  (CallFunction|NewVector _output_get "25.000000,25.000000,-25.000000" "50.000000,50.000000,25.000000")
  (switch Utilities|FlowControl|Switch|SwitchonE_QuestionType (Variables|Default|GetQuestionType)
    (:NewEnumerator0
      (bind _returnvalue_5 (Game|SpawnActorfromClass "/Game/BP_QuestionVector.BP_QuestionVector_C" (Math|Transform|MakeTransform (+ (Transformation|GetActorLocation _output_get) (Variables|/Game/BP_QuestionVector.BP_QuestionVector_C|GetVector%20End _output_get)) "0, 0, 0" "1.000000,1.000000,1.000000") "Undefined" 0 "(R=0.000000,G=0.000000,B=1.000000,A=1.000000)" 0 :!label _label))
      (bind _output_get_2 (Variables|Default|SetVector%202 _returnvalue_5))
      (CallFunction|NewVector _output_get_2 "25.000000,-25.000000,25.000000" "50.000000,0.000000,50.000000"))
    (:NewEnumerator1
      (goto _label))
    (:NewEnumerator2
      (Variables|Default|SetScalarMul (Math|Random|RandomFloatinRange -2.0 2.0)))
    (:NewEnumerator3
      (bind _returnvalue_6 (Game|SpawnActorfromClass "/Game/BP_QuestionVector.BP_QuestionVector_C" (Math|Transform|MakeTransform _returnvalue "0, 0, 0" "1.000000,1.000000,1.000000") "Undefined" 0 "(R=0.000000,G=0.000000,B=1.000000,A=1.000000)" 0))
      (bind _output_get_3 (Variables|Default|SetVector%202 _returnvalue_6))
      (CallFunction|NewVector _output_get_3 "25.000000,-25.000000,25.000000" "50.000000,0.000000,50.000000")))
  (EventDispatchers|BindEventtoCheckAnswer (Variables|Default|GetAnswerVector) (EventDispatchers|CreateEvent :!event CheckAnswer))
  (switch Utilities|FlowControl|Switch|SwitchonE_QuestionType (Variables|Default|GetQuestionType)
    (:NewEnumerator0
      (Variables|Default|SetVectorAnswer (+ (Transformation|GetActorLocation (Variables|Default|GetVector%201)) (Variables|/Game/BP_QuestionVector.BP_QuestionVector_C|GetVector%20End (Variables|Default|GetVector%201)) (Variables|/Game/BP_QuestionVector.BP_QuestionVector_C|GetVector%20End (Variables|Default|GetVector%202)))))
    (:NewEnumerator1
      (Variables|Default|SetVectorAnswer (- (+ (Transformation|GetActorLocation (Variables|Default|GetVector%201)) (Variables|/Game/BP_QuestionVector.BP_QuestionVector_C|GetVector%20End (Variables|Default|GetVector%201))) (Variables|/Game/BP_QuestionVector.BP_QuestionVector_C|GetVector%20End (Variables|Default|GetVector%202)))))
    (:NewEnumerator2
      (Variables|Default|SetVectorAnswer (+ (Transformation|GetActorLocation (Variables|Default|GetVector%201)) (* (Variables|/Game/BP_QuestionVector.BP_QuestionVector_C|GetVector%20End (Variables|Default|GetVector%201)) (Variables|Default|GetScalarMul)))))
    (:NewEnumerator3
      (Variables|Default|SetVectorAnswer (Math|Vector|CrossProduct (Variables|/Game/BP_QuestionVector.BP_QuestionVector_C|GetVector%20End (Variables|Default|GetVector%201)) (* (Variables|/Game/BP_QuestionVector.BP_QuestionVector_C|GetVector%20End (Variables|Default|GetVector%202)) -1.0))))))

(fn ConstructionScript)

(fn NewVector
  (params (VectorActor :type BP%20Question%20Vector%20Object%20Reference) (Min :type Vector) (Max :type Vector))
  (bind _arrowx (Variables|/Game/BP_QuestionVector.BP_QuestionVector_C|GetArrowX VectorActor))
  (bind _output_get (Variables|/Game/BP_QuestionVector.BP_QuestionVector_C|SetVector%20End VectorActor (Math|Vector|MakeVector (Math|Random|RandomFloatinRange (.x Min) (.x Max)) (Math|Random|RandomFloatinRange (.y Min) (.y Max)) (Math|Random|RandomFloatinRange (.z Min) (.z Max)))))
  (Variables|/Script/Engine.ArrowComponent|SetArrowLength _arrowx (Math|Vector|VectorLength _output_get))
  (Components|Arrow|SetArrowColor(LinearColor) _arrowx (Math|Conversions|ToLinearColor(Color) (Variables|/Script/Engine.ArrowComponent|GetArrowColor _arrowx)))
  (Transformation|SetWorldRotation _arrowx (Math|Vector|RotatorfromAxisandAngle "0.000000,0.000000,1.000000" (Class|KismetMathLibrary|DegAtan2 (.Y (Class|KismetMathLibrary|BreakVector3f _output_get)) (.X (Class|KismetMathLibrary|BreakVector3f _output_get)))) false false)
  (Transformation|AddWorldRotation _arrowx (Math|Vector|RotatorfromAxisandAngle (Math|Vector|Normalize (Math|Vector|MakeVector (.Y (Class|KismetMathLibrary|BreakVector3f _output_get)) (* (.X (Class|KismetMathLibrary|BreakVector3f _output_get)) -1.0) 0.0)) (Class|KismetMathLibrary|DegAtan2 (.Z (Class|KismetMathLibrary|BreakVector3f _output_get)) (Class|KismetMathLibrary|Hypotenuse (.X (Class|KismetMathLibrary|BreakVector3f _output_get)) (.Y (Class|KismetMathLibrary|BreakVector3f _output_get))))) false false))

(fn CheckAnswer
  (params (Answer%20Vector%20End :type Vector))
  (bind _vectoranswer (Variables|Default|GetVectorAnswer))
  (bind _vectoranswer_2 (Variables|Default|GetVectorAnswer))
  (bind _vector_1 (Variables|Default|GetVector%201))
  (bind _returnvalue (Class|KismetMathLibrary|VectorDistanceSquared Answer%20Vector%20End _vectoranswer_2))
  (bind _returnvalue_2 (Math|Vector|Normalize _vectoranswer))
  (bind _returnvalue_3 (Transformation|GetActorLocation _vector_1))
  (bind _returnvalue_4 (- Answer%20Vector%20End _returnvalue_3))
  (bind _returnvalue_5 (Math|Vector|Normalize _returnvalue_4))
  (bind _returnvalue_6 (Math|Vector|DotProduct _returnvalue_5 _returnvalue_2))
  (switch Utilities|FlowControl|Switch|SwitchonE_QuestionType (Variables|Default|GetQuestionType)
    (:NewEnumerator0
      (Development|PrintString (Utilities|String|ToString(Float) _returnvalue) :!label _label)
      (if (< _returnvalue 5e+01)
        (Utilities|FlowControl|DoOnce false :!label _label_2
          (:Completed
            (Default|CallCheckAnswerDispatch)))))
    (:NewEnumerator1
      (goto _label))
    (:NewEnumerator2
      (goto _label))
    (:NewEnumerator3
      (Development|PrintString (Utilities|String|ToString(Float) _returnvalue_6))
      (if (> _returnvalue_6 0.9)
        (goto _label_2)))))

(fn ArbitraryVector
  (params (VectorActor :type BP%20Question%20Vector%20Object%20Reference) (Vector :type Vector))
  (bind _arrowx (Variables|/Game/BP_QuestionVector.BP_QuestionVector_C|GetArrowX VectorActor))
  (bind _output_get (Variables|/Game/BP_QuestionVector.BP_QuestionVector_C|SetVector%20End VectorActor Vector))
  (Variables|/Script/Engine.ArrowComponent|SetArrowLength _arrowx (Math|Vector|VectorLength _output_get))
  (Components|Arrow|SetArrowColor(LinearColor) _arrowx (Math|Conversions|ToLinearColor(Color) (Variables|/Script/Engine.ArrowComponent|GetArrowColor _arrowx)))
  (Transformation|SetWorldRotation _arrowx (Math|Vector|RotatorfromAxisandAngle "0.000000,0.000000,1.000000" (Class|KismetMathLibrary|DegAtan2 (.Y (Class|KismetMathLibrary|BreakVector3f _output_get)) (.X (Class|KismetMathLibrary|BreakVector3f _output_get)))) false false)
  (Transformation|AddWorldRotation _arrowx (Math|Vector|RotatorfromAxisandAngle (Math|Vector|Normalize (Math|Vector|MakeVector (.Y (Class|KismetMathLibrary|BreakVector3f _output_get)) (* (.X (Class|KismetMathLibrary|BreakVector3f _output_get)) -1.0) 0.0)) (Class|KismetMathLibrary|DegAtan2 (.Z (Class|KismetMathLibrary|BreakVector3f _output_get)) (Class|KismetMathLibrary|Hypotenuse (.X (Class|KismetMathLibrary|BreakVector3f _output_get)) (.Y (Class|KismetMathLibrary|BreakVector3f _output_get))))) false false))

(fn RemoveSelf
  (Actor|DestroyActor (Variables|Default|GetVector%201)))