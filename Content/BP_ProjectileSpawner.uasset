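; BP_ProjectileSpawner spawns throwable projectiles at its own location, choosing their class from the battle mode's throw setting.
; On BeginPlay it reads ThrowMode from GI_battlemode and spawns BP_ProjectileAxis for Axis mode, or BP_Projectile for Direct, Addition and Cross.
; Each projectile receives the mode and PlayerDetector as owner, then binds back to Spawnagain so the projectile itself triggers the next spawn.
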(event Custom|Spawnagain
  (bind _returnvalue (Transformation|GetActorLocation))
  (bind _player_detector (Variables|Default|Getplayer_detector))
  (bind _projectile_mode (Variables|Default|GetProjectile%20Mode))
  (switch Utilities|FlowControl|Switch|SwitchonE_ProjectileMode _projectile_mode
    (:NewEnumerator0
      (bind _returnvalue_2 (Game|SpawnActorfromClass "/Game/BP_Projectile.BP_Projectile_C" (Math|Transform|MakeTransform _returnvalue "0, 0, 0" "1.000000,1.000000,1.000000") "Undefined" 0 _projectile_mode 0 :!label _label))
      (Variables|/Game/BP_Projectile.BP_Projectile_C|SetProjectile_owner _returnvalue_2 _player_detector)
      (EventDispatchers|BindEventtoSpawnAgain _returnvalue_2 (delegate Custom|Spawnagain)))
    (:NewEnumerator1
      (bind _returnvalue_3 (Game|SpawnActorfromClass "/Game/BP_ProjectileAxis.BP_ProjectileAxis_C" (Math|Transform|MakeTransform _returnvalue "0, 0, 0" "1.000000,1.000000,1.000000") "Undefined" 0 _projectile_mode 0))
      (Variables|/Game/BP_Projectile.BP_Projectile_C|SetProjectile_owner _returnvalue_3 _player_detector)
      (EventDispatchers|BindEventtoSpawnAgain _returnvalue_3 (delegate Custom|Spawnagain)))
    (:NewEnumerator2
      (goto _label))
    (:NewEnumerator3
      (goto _label))))

(event EventBeginPlay
  (bind _asgi_battlemode (Utilities|Casting|CastToGI_battlemode (Game|GetGameInstance)))
  (Variables|Default|SetProjectile%20Mode (Variables|/Game/GI_battlemode.GI_battlemode_C|GetThrow_mode _asgi_battlemode))
  (CallFunction|Spawnagain))

(fn ConstructionScript)