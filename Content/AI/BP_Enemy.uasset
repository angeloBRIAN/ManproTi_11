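; BP_Enemy is an AI enemy that fires physics-driven BP_Projectile actors from its ShootDir point and turns on mesh physics once Health reaches zero.
; ShootPlayer fires along the enemy's rotation, and ShootPlayerMiss offsets the yaw to miss deliberately.
; ShootPlayerPredict rotates the projectile toward a velocity-led player position, but its impulse points at the player's current location.
; Tick polls Health, and no caller of the shoot events appears here.
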(event Custom|ShootPlayerPredict
  (bind _returnvalue (Game|GetPlayerCharacter 0))
  (Utilities|IsValid _returnvalue
    (:Is%20Valid
      (bind _returnvalue_2 (Game|SpawnActorfromClass "/Game/BP_Projectile.BP_Projectile_C" (Math|Transform|MakeTransform (Transformation|GetWorldLocation (Variables|Default|GetShootDir)) (Math|Rotator|FindLookatRotation (Transformation|GetWorldLocation (Variables|Default|GetShootDir)) (+ (+ (Transformation|GetActorLocation _returnvalue) "0.000000,0.000000,80.000000") (* (Transformation|GetVelocity _returnvalue) (/ (Transformation|GetDistanceTo _returnvalue) (Variables|Default|GetBulletSpeed))))) "1.000000,1.000000,1.000000") "Undefined" 0 "NewEnumerator0" 0))
      (Physics|SetSimulatePhysics (Variables|/Game/BP_Projectile.BP_Projectile_C|GetSphere _returnvalue_2) true)
      (Physics|AddImpulse (Variables|/Game/BP_Projectile.BP_Projectile_C|GetSphere _returnvalue_2) (* (- (Transformation|GetActorLocation (Game|GetPlayerCharacter 0)) (Transformation|GetActorLocation _returnvalue_2)) (Variables|Default|GetBulletSpeed)) "None" true))))

(event Custom|ShootPlayerMiss
  (bind _returnvalue (Transformation|GetActorRotation))
  (bind _bulletspeed (Variables|Default|GetBulletSpeed))
  (bind _returnvalue_2 (Game|SpawnActorfromClass "/Game/BP_Projectile.BP_Projectile_C" (Math|Transform|MakeTransform (Transformation|GetWorldLocation (Variables|Default|GetShootDir)) (Math|Rotator|MakeRotator (.roll _returnvalue) (.pitch _returnvalue) (+ (.yaw _returnvalue) 3e+01))) "Undefined" 0 "NewEnumerator0" 0))
  (Variables|/Game/BP_Projectile.BP_Projectile_C|SetProjectile_owner _returnvalue_2 self)
  (Class|PrimitiveComponent|SetAllPhysicsLinearVelocity (Variables|/Game/BP_Projectile.BP_Projectile_C|GetSphere _returnvalue_2) (* (Variables|Default|Getvelocity_awal) _bulletspeed) true)
  (Physics|SetSimulatePhysics (Variables|/Game/BP_Projectile.BP_Projectile_C|GetSphere _returnvalue_2) true)
  (Physics|AddForce (Variables|/Game/BP_Projectile.BP_Projectile_C|GetSphere _returnvalue_2) (Math|Vector|MakeVector _bulletspeed 0.0 0.0) "None" true)
  (Default|DestroyArrow _returnvalue_2))

(event Custom|ShootPlayer
  (bind _bulletspeed (Variables|Default|GetBulletSpeed))
  (bind _returnvalue (Game|SpawnActorfromClass "/Game/BP_Projectile.BP_Projectile_C" (Math|Transform|MakeTransform (Transformation|GetWorldLocation (Variables|Default|GetShootDir)) (Transformation|GetActorRotation)) "Undefined" 0 "NewEnumerator0" 0))
  (Variables|/Game/BP_Projectile.BP_Projectile_C|SetProjectile_owner _returnvalue self)
  (Class|PrimitiveComponent|SetAllPhysicsLinearVelocity (Variables|/Game/BP_Projectile.BP_Projectile_C|GetSphere _returnvalue) (* (Variables|Default|Getvelocity_awal) _bulletspeed) true)
  (Physics|SetSimulatePhysics (Variables|/Game/BP_Projectile.BP_Projectile_C|GetSphere _returnvalue) true)
  (Physics|AddForce (Variables|/Game/BP_Projectile.BP_Projectile_C|GetSphere _returnvalue) (Math|Vector|MakeVector _bulletspeed 0.0 0.0) "None" true)
  (Default|DestroyArrow _returnvalue))

(event EventTick
  (params (DeltaSeconds :type Float%20%28single-precision%29))
  (if (<= (Variables|Default|GetHealth) 0.0)
    (Physics|SetSimulatePhysics (Variables|Character|GetMesh) true)))

(event Collision|EventActorBeginOverlap
  (params (OtherActor :type Actor%20Object%20Reference)))

(fn ConstructionScript)