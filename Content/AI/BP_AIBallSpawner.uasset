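; BP_AIBallSpawner is an actor that populates the area around itself with BP_Ball actors.
; After BeginPlay it enables Tick, which attempts one spawn per frame until the spawn counter reaches BallCount.
; X and Y come from separate random reachable-point queries around the spawner, while Z is fixed.
; The delayed counter decrement and player-distance check are unconnected, so spawning never replenishes.
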(event Custom|SpawnBall
  (bind _returnvalue (Transformation|GetActorLocation))
  (bind _randomlocation (AI|Navigation|GetRandomReachablePointinRadius _returnvalue 5e+02 0 0))
  (bind _returnvalue_2 (Game|SpawnActorfromClass "/Game/AI/BP_Ball.BP_Ball_C" (Math|Transform|MakeTransform (Math|Vector|MakeVector (.x _randomlocation) (.y _randomlocation) -3.5e+02) "0, 0, 0" "1.000000,1.000000,1.000000") "Undefined" 0 0))
  (Utilities|IsValid _returnvalue_2
    (:Is%20Valid
      (Math|Integer|IncrementInt (Variables|Default|GetSpawnBallCount)))))

(event EventBeginPlay
  (Utilities|FlowControl|Delay 0.0)
  (Actor|Tick|SetActorTickEnabled true))

(event EventTick
  (params (DeltaSeconds :type Float%20%28single-precision%29))
  (if (< (Variables|Default|GetSpawnBallCount) (Variables|Default|GetBallCount))
    (CallFunction|SpawnBall)
    (Development|PrintString "Ball Spawned")))

(fn ConstructionScript)