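; BP_ProjectileAxis is a physics sphere projectile launched along a vector built from three axis handles.
; On BeginPlay it spawns and attaches three rotated, color-coded BP_VectorAxis actors, one per axis.
; Drop detaches it and enables physics; if any handle moved, it combines one coordinate from each head into a scaled, mass-independent impulse.
; It then destroys the handles, starts a self-destruct timer and plays a sound.
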(event EventBeginPlay
  (bind _returnvalue (Game|SpawnActorfromClass "/Game/BP_VectorAxis.BP_VectorAxis_C" (Math|Transform|MakeTransform "0, 0, 0" "0, 0, 0" "1.000000,1.000000,1.000000") "Undefined" 0 "(R=1.000000,G=0.000000,B=0.000000,A=1.000000)" 4e+01 "NewEnumerator0" 0))
  (Utilities|Array|Add (Variables|Default|GetVectors) _returnvalue)
  (Transformation|AttachActorToActor _returnvalue self "" "KeepRelative" "KeepRelative" "KeepRelative" true)
  (bind _returnvalue_2 (Game|SpawnActorfromClass "/Game/BP_VectorAxis.BP_VectorAxis_C" (Math|Transform|MakeTransform "0, 0, 0" "0.000000,90.000000,0.000000" "1.000000,1.000000,1.000000") "Undefined" 0 "(R=0.000000,G=1.000000,B=0.000000,A=1.000000)" 4e+01 "NewEnumerator1" 0))
  (Utilities|Array|Add (Variables|Default|GetVectors) _returnvalue_2)
  (Transformation|AttachActorToActor _returnvalue_2 self "" "KeepRelative" "KeepRelative" "KeepRelative" true)
  (bind _returnvalue_3 (Game|SpawnActorfromClass "/Game/BP_VectorAxis.BP_VectorAxis_C" (Math|Transform|MakeTransform "0, 0, 0" "90.000000,0.000000,0.000000" "1.000000,1.000000,1.000000") "Undefined" 0 "(R=0.000000,G=0.000000,B=1.000000,A=1.000000)" 4e+01 "NewEnumerator2" 0))
  (Utilities|Array|Add (Variables|Default|GetVectors) _returnvalue_3)
  (Transformation|AttachActorToActor _returnvalue_3 self "" "KeepRelative" "KeepRelative" "KeepRelative" true))

(event EventDestroyArrow
  (for _array_element (Variables|Default|GetVectors)
    (Transformation|DetachFromActor _array_element "KeepRelative" "KeepRelative" "KeepRelative")
    (Actor|DestroyActor _array_element)
    (CallFunction|DestroySelfTimer)))

(event EventDrop
  (bind _vectors (Variables|Default|GetVectors))
  (bind _output (Utilities|Array|Get(acopy) _vectors 2))
  (bind _output_2 (Utilities|Array|Get(acopy) _vectors))
  (bind _output_3 (Utilities|Array|Get(acopy) _vectors 1))
  (Transformation|DetachFromActor "KeepWorld" "KeepWorld" "KeepRelative")
  (Physics|SetSimulatePhysics (Variables|Default|GetSphere) true)
  (if (Math|Boolean|ORBoolean (Variables|/Game/BP_VectorAxis.BP_VectorAxis_C|GetIsVectorMoved _output_2) (Variables|/Game/BP_VectorAxis.BP_VectorAxis_C|GetIsVectorMoved _output_3) (Variables|/Game/BP_VectorAxis.BP_VectorAxis_C|GetIsVectorMoved _output))
    (Physics|AddImpulse (Variables|Default|GetSphere) (* (- (Math|Vector|MakeVector (.X (Math|Vector|BreakVector (Variables|/Game/BP_VectorAxis.BP_VectorAxis_C|GetVector%20Head%20Loc _output_2))) (.Y (Math|Vector|BreakVector (Variables|/Game/BP_VectorAxis.BP_VectorAxis_C|GetVector%20Head%20Loc _output_3))) (.Z (Math|Vector|BreakVector (Variables|/Game/BP_VectorAxis.BP_VectorAxis_C|GetVector%20Head%20Loc _output)))) (Transformation|GetActorLocation)) 1e+01) "None" true))
  (CallFunction|DestroyArrow)
  (CallFunction|DestroySelfTimer)
  (Audio|PlaySoundatLocation "/Game/SoundEffect/sthswng1.sthswng1" (Transformation|GetActorLocation) "0, 0, 0" 1.0 1.0 0.0 0 0 0 0))

(fn ConstructionScript
  (|CallParentFunction))