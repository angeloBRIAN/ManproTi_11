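; Vector answer actor: an arrow the player shapes by finger position to submit as an answer.
; MoveVectorHead moves the sphere to the finger, sets arrow length, and rotates the actor by yaw, then elevation, using Atan2 angles.
; Tick displays length and both angles and recomputes the head's world location, which CheckAnswer_Intermediary passes to CallCheckAnswer.
; Helpers destroy the sphere or compute a head offset; Pickup and Drop are empty.
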(event Custom|CheckAnswer_Intermediary
  (Default|CallCheckAnswer (Variables|Default|GetVector%20Head%20Loc)))

(event EventBeginPlay
  (bind _vectorarrow (Variables|Default|GetVectorArrow))
  (bind _output_get (Variables|/Script/Engine.ArrowComponent|SetArrowLength _vectorarrow (Variables|Default|GetVector%20Length)))
  (Components|Arrow|SetArrowColor(LinearColor) _vectorarrow (Variables|Default|GetVector%20Color)))

(event EventDrop)

(event EventTick
  (params (DeltaSeconds :type Float%20%28single-precision%29))
  (Rendering|Components|TextRender|SetText (Variables|Default|GetDisplay) (Utilities|Text|FormatText "{0}, {1}°, {2}°" (Variables|/Script/Engine.ArrowComponent|GetArrowLength (Variables|Default|GetVectorArrow)) (Utilities|Text|ToText(Float) (Variables|Default|GetAngle%20XY) "HalfToEven" false true 1 324 0 1) (Utilities|Text|ToText(Float) (Variables|Default|GetAngle%20Z) "HalfToEven" false true 1 324 0 1)))
  (Variables|Default|SetVector%20Head%20Loc (+ (Transformation|GetActorLocation) (Math|Vector|RotateVector (Math|Vector|MakeVector (stale EventBeginPlay _output_get) 0.0 0.0) (Transformation|GetActorRotation)))))

(event EventPickup
  (params (Attach%20To :type Scene%20Component%20Object%20Reference)))

(fn ConstructionScript)

(fn MoveVectorHead
  (params (FingerPos :type Vector))
  (bind _returnvalue (Transformation|GetActorLocation))
  (bind _vectorarrow (Variables|Default|GetVectorArrow))
  (bind _returnvalue_2 (- FingerPos _returnvalue))
  (Variables|/Script/Engine.ArrowComponent|SetArrowLength _vectorarrow (Math|Vector|Distance(Vector) FingerPos _returnvalue))
  (Components|Arrow|SetArrowColor(LinearColor) _vectorarrow (Math|Conversions|ToLinearColor(Color) (Variables|/Script/Engine.ArrowComponent|GetArrowColor _vectorarrow)))
  (Transformation|SetWorldLocation (Variables|Default|GetSphere) FingerPos false false)
  (bind _output_get (Variables|Default|SetAngle%20XY (Class|KismetMathLibrary|DegAtan2 (.y _returnvalue_2) (.x _returnvalue_2))))
  (Transformation|SetActorRotation (Math|Vector|RotatorfromAxisandAngle "0.000000,0.000000,1.000000" _output_get))
  (bind _output_get_2 (Variables|Default|SetAngle%20Z (Class|KismetMathLibrary|DegAtan2 (.z _returnvalue_2) (Class|KismetMathLibrary|Hypotenuse (.x _returnvalue_2) (.y _returnvalue_2)))))
  (Class|Actor|AddActorWorldRotation (Math|Vector|RotatorfromAxisandAngle (Math|Vector|Normalize (Math|Vector|MakeVector (.y _returnvalue_2) (* (.x _returnvalue_2) -1.0) 0.0)) _output_get_2))
  (Variables|Default|SetIsVectorMoved true))

(fn DestroySphere
  (Components|DestroyComponent (Variables|Default|GetSphere)))

(fn GetArrowHeadLoc
  (bind _vectorarrow (Variables|Default|GetVectorArrow))
  (bind _returnvalue (Transformation|GetWorldRotation _vectorarrow))
  (return (* (Math|Vector|MakeVector (Math|Trig|Cos(Degrees) (.yaw _returnvalue)) (Math|Trig|Sin(Degrees) (.yaw _returnvalue)) (Math|Trig|Sin(Degrees) (.pitch _returnvalue))) (Variables|/Script/Engine.ArrowComponent|GetArrowLength _vectorarrow))))