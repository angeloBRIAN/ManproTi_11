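; Development control actor that uses keyboard keys to move a Cube and a Sphere and test grab and pinch interactions, apparently standing in for two hands.
; WASD/Space/Shift nudge the Cube and numpad/Enter nudge the Sphere in fixed world steps.
; Q toggles picking up and dropping overlapped I_Pickup actors through interface messages.
; NumPad 7 toggles pinching, which each Tick drags a held BP_VectorAnswer or BP_VectorAxis head to Scene1's location.
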(event EventBeginPlay)

(event Collision|EventActorBeginOverlap
  (params (OtherActor :type Actor%20Object%20Reference)))

(event EventTick
  (params (DeltaSeconds :type Float%20%28single-precision%29))
  (if (Variables|Default|GetPinched)
    (CallFunction|MoveVectorHeadd)))

(event Input|KeyboardEvents|NumPadFour
  (params (Key :type Key%20Structure :default "None"))
  (:Pressed
    (Transformation|AddWorldOffset (Variables|Default|GetSphere) "0.000000,-10.000000,0.000000" false false)))

(event Input|KeyboardEvents|NumPadSix
  (params (Key :type Key%20Structure :default "None"))
  (:Pressed
    (Transformation|AddWorldOffset (Variables|Default|GetSphere) "0.000000,10.000000,0.000000" false false)))

(event Input|KeyboardEvents|Enter
  (params (Key :type Key%20Structure :default "None"))
  (:Pressed
    (Transformation|AddWorldOffset (Variables|Default|GetSphere) "0.000000,0.000000,-10.000000" false false)))

(event Input|KeyboardEvents|NumPadZero
  (params (Key :type Key%20Structure :default "None"))
  (:Pressed
    (Transformation|AddWorldOffset (Variables|Default|GetSphere) "0.000000,0.000000,10.000000" false false)))

(event Input|KeyboardEvents|Q
  (params (Key :type Key%20Structure :default "None"))
  (:Pressed
    (Utilities|FlowControl|FlipFlop
      (:A
        (CallFunction|Grab))
      (:B
        (CallFunction|Release)))))

(event Input|KeyboardEvents|NumPadSeven
  (params (Key :type Key%20Structure :default "None"))
  (:Pressed
    (Variables|Default|SetPinched (not (Variables|Default|GetPinched)))
    (Utilities|FlowControl|FlipFlop
      (:A
        (CallFunction|Pinch))
      (:B
        (CallFunction|Unpinch)))))

(event Input|KeyboardEvents|W
  (params (Key :type Key%20Structure :default "None"))
  (:Pressed
    (Transformation|AddWorldOffset (Variables|Default|GetCube) "10.000000,0.000000,0.000000" false false)))

(event Input|KeyboardEvents|A
  (params (Key :type Key%20Structure :default "None"))
  (:Pressed
    (Transformation|AddWorldOffset (Variables|Default|GetCube) "0.000000,-10.000000,0.000000" false false)))

(event Input|KeyboardEvents|S
  (params (Key :type Key%20Structure :default "None"))
  (:Pressed
    (Transformation|AddWorldOffset (Variables|Default|GetCube) "-10.000000,0.000000,0.000000" false false)))

(event Input|KeyboardEvents|D
  (params (Key :type Key%20Structure :default "None"))
  (:Pressed
    (Transformation|AddWorldOffset (Variables|Default|GetCube) "0.000000,10.000000,0.000000" false false)))

(event Input|KeyboardEvents|LeftShift
  (params (Key :type Key%20Structure :default "None"))
  (:Pressed
    (Transformation|AddWorldOffset (Variables|Default|GetCube) "0.000000,0.000000,-10.000000" false false)))

(event Input|KeyboardEvents|SpaceBar
  (params (Key :type Key%20Structure :default "None"))
  (:Pressed
    (Transformation|AddWorldOffset (Variables|Default|GetCube) "0.000000,0.000000,10.000000" false false)))

(event Input|KeyboardEvents|NumPadEight
  (params (Key :type Key%20Structure :default "None"))
  (:Pressed
    (Transformation|AddWorldOffset (Variables|Default|GetSphere) "10.000000,0.000000,0.000000" false false)))

(event Input|KeyboardEvents|NumPadFive
  (params (Key :type Key%20Structure :default "None"))
  (:Pressed
    (Transformation|AddWorldOffset (Variables|Default|GetSphere) "-10.000000,0.000000,0.000000" false false)))

(fn ConstructionScript)

(fn Grab
  (bind _array_element (Utilities|Array|ForEachLoopwithBreak (Collision|GetOverlappingActors (Variables|Default|GetSphereC) 0 :!class /Script/Engine.PrimitiveComponent) :!label _label)
    (:LoopBody
      (Development|PrintString (Utilities|GetDisplayName _array_element))
      (if (Utilities|DoesObjectImplementInterface _array_element "/Game/I_Pickup.I_Pickup_C")
        (Variables|Default|SetAttachedObjectL _array_element)
        (Class|IPickup|Pickup(Message) _array_element (Variables|Default|GetScene))
        (goto _label Break)))))

(fn Release
  (bind _attachedobjectl (Variables|Default|GetAttachedObjectL)
    (:then
      (if (== (Transformation|GetAttachParent (Variables|/Script/Engine.Actor|GetRootComponent _attachedobjectl)) (Variables|Default|GetScene))
        (Class|IPickup|Drop(Message) _attachedobjectl)
        (Variables|Default|SetAttachedObjectL 0)))
    (:else)))

(fn Pinch
  (bind _array_element (Utilities|Array|ForEachLoopwithBreak (Collision|GetOverlappingActors (Variables|Default|GetSphereC1) 0 :!class /Script/Engine.PrimitiveComponent) :!label _label)
    (:LoopBody
      (Development|PrintString (Utilities|GetDisplayName _array_element))
      (if (Utilities|DoesObjectImplementInterface _array_element "/Game/I_Pickup.I_Pickup_C")
        (Variables|Default|SetAttachedObjectR _array_element)
        (goto _label Break)))))

(fn Unpinch
  (Variables|Default|SetAttachedObjectR 0))

(fn MoveVectorHeadd
  (bind _scene1 (Variables|Default|GetScene1))
  (bind _returnvalue (Transformation|GetWorldLocation _scene1))
  (bind _attachedobjectr (Variables|Default|GetAttachedObjectR)
    (:then
      (if (Variables|Default|GetPinched)
        (bind _asbp_vector_answer (Utilities|Casting|CastToBP_VectorAnswer _attachedobjectr)
          (:then
            (Default|MoveVectorHead _asbp_vector_answer _returnvalue))
          (:CastFailed
            (bind _asbp_vector_axis (Utilities|Casting|CastToBP_VectorAxis _attachedobjectr))
            (Default|MoveVectorHead _asbp_vector_axis _returnvalue)))))
    (:else)))