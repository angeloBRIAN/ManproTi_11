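; Manager actor for a free-mode vector math sandbox covering addition, subtraction, scalar multiplication, dot and cross products.
; Spawns input vectors A and B plus result C, and takes operation and scalar changes from WB_OperationSelector dispatchers.
; Tick recomputes C or the dot-product text, gating all but scalar mode on A/B endpoint proximity.
; Returning to the main menu destroys the vectors, fades the selector, removes the menu's grids and destroys itself.
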(event Custom|Spawn%20Vectors
  (bind _returnvalue (Transformation|GetActorTransform))
  (bind _returnvalue_2 (Math|Rotator|CombineRotators (.rotation _returnvalue) "0.000000,-90.000000,0.000000"))
  (bind _returnvalue_3 (Game|SpawnActorfromClass "/Game/_PRACTICE/BP_VectorAnswer_NEW.BP_VectorAnswer_NEW_C" (Math|Transform|MakeTransform (.location _returnvalue) _returnvalue_2 "1.000000,1.000000,1.000000") "Undefined" 0 "(R=1.000000,G=0.000000,B=0.000000,A=1.000000)" 4e+01 "A" 0))
  (Variables|Default|SetVector%201 _returnvalue_3)
  (bind _returnvalue_4 (Game|SpawnActorfromClass "/Game/_PRACTICE/BP_VectorAnswer_NEW.BP_VectorAnswer_NEW_C" (Math|Transform|MakeTransform (+ (.location _returnvalue) "0.000000,0.000000,20.000000") _returnvalue_2 "1.000000,1.000000,1.000000") "Undefined" 0 "(R=0.000000,G=1.000000,B=0.000000,A=1.000000)" 4e+01 "B" 0))
  (Variables|Default|SetVector%202 _returnvalue_4)
  (bind _returnvalue_5 (Game|SpawnActorfromClass "/Game/_PRACTICE/BP_VectorDisplay.BP_VectorDisplay_C" (Math|Transform|MakeTransform "0.000000,0.000000,-500.000000" "0, 0, 0" "1.000000,1.000000,1.000000") "Undefined" 0 "(R=0.000000,G=0.000000,B=1.000000,A=1.000000)" 4e+01 "C" 0))
  (Variables|Default|SetVector%203 _returnvalue_5))

(event Custom|Modify%20Scalar
  (params (Scalar :type Float%20%28double-precision%29))
  (Variables|Default|SetScalar (+ (Variables|Default|GetScalar) Scalar)))

(event Custom|Return%20to%20Main%20Menu
  (bind _returnvalue (Game|GetGameInstance))
  (bind _asgi_new (Utilities|Casting|CastToGI_NEW _returnvalue))
  (bind _main_menu (Variables|/Game/_MAIN_MENU/GI_NEW.GI_NEW_C|GetMain%20Menu _asgi_new))
  (Actor|DestroyActor (Variables|Default|GetVector%201))
  (bind _awd (Timeline|timerShowMenu PlayFromStart)
    (:Update
      (Widget|SetRenderOpacity (UserInterface|GetUserWidgetObject (Variables|Default|GetMode%20Selector)) _awd))
    (:Finished
      (Widget|SetRenderOpacity (UserInterface|GetUserWidgetObject (Variables|/Game/_MAIN_MENU/BP_MainMenu.BP_MainMenu_C|GetMainMenuWidget _main_menu)) 1.0)
      (Default|ShowMainMenu _main_menu)
      (for _array_element (Variables|/Game/_MAIN_MENU/BP_MainMenu.BP_MainMenu_C|GetGrids _main_menu)
        (Actor|DestroyActor _array_element))
      (Actor|DestroyActor (Variables|/Game/_MAIN_MENU/BP_MainMenu.BP_MainMenu_C|GetGridZero _main_menu))
      (Actor|DestroyActor))))

(event Custom|Change%20Operation
  (params (Question%20Type :type E_QuestionType%20Enum :default "NewEnumerator0"))
  (bind _returnvalue (Transformation|GetActorTransform))
  (bind _vector_3 (Variables|Default|GetVector%203))
  (bind _returnvalue_2 (Math|Rotator|CombineRotators (.rotation _returnvalue) "0.000000,-90.000000,0.000000"))
  (bind _defaultsceneroot (Variables|/Game/_PRACTICE/BP_VectorDisplay.BP_VectorDisplay_C|GetDefaultSceneRoot _vector_3))
  (Variables|Default|SetQuestion%20Type Question%20Type)
  (Variables|Default|SetStartCheck true)
  (Transformation|SetActorLocationAndRotation (Variables|Default|GetVector%201) (.location _returnvalue) _returnvalue_2)
  (Transformation|SetActorLocationAndRotation (Variables|Default|GetVector%202) (+ (.location _returnvalue) "0.000000,0.000000,20.000000") _returnvalue_2)
  (switch Utilities|FlowControl|Switch|SwitchonE_QuestionType (Variables|Default|GetQuestion%20Type)
    (:NewEnumerator0
      (Rendering|SetVisibility _defaultsceneroot true true :!label _label))
    (:NewEnumerator1
      (goto _label))
    (:NewEnumerator2
      (CallFunction|HideSecondVector)
      (goto _label))
    (:NewEnumerator4
      (Rendering|SetVisibility _defaultsceneroot false true))
    (:NewEnumerator3
      (goto _label))))

(event EventTick
  (params (DeltaSeconds :type Float%20%28single-precision%29))
  (bind _vector_3 (Variables|Default|GetVector%203))
  (bind _vector_3_2 (Variables|Default|GetVector%203))
  (bind _vector_1 (Variables|Default|GetVector%201))
  (bind _vector_2 (Variables|Default|GetVector%202))
  (bind _vector_3_3 (Variables|Default|GetVector%203))
  (bind _vector_1_2 (Variables|Default|GetVector%201))
  (bind _vector_3_4 (Variables|Default|GetVector%203))
  (bind _mode_selector (Variables|Default|GetMode%20Selector))
  (bind _vector_3_5 (Variables|Default|GetVector%203))
  (bind _returnvalue (Transformation|GetActorLocation _vector_1))
  (bind _returnvalue_2 (Transformation|GetActorLocation _vector_1_2))
  (bind _returnvalue_3 (UserInterface|GetUserWidgetObject _mode_selector))
  (bind _defaultsceneroot (Variables|/Game/_PRACTICE/BP_VectorAnswer_NEW.BP_VectorAnswer_NEW_C|GetDefaultSceneRoot _vector_1_2))
  (bind _defaultsceneroot_2 (Variables|/Game/_PRACTICE/BP_VectorDisplay.BP_VectorDisplay_C|GetDefaultSceneRoot _vector_3_5))
  (bind _returnvalue_4 (Math|Vector|GetUpVector _defaultsceneroot))
  (bind _aswb_operation_selector (Utilities|Casting|CastToWB_OperationSelector _returnvalue_3))
  (bind _returnvalue_5 (* _returnvalue_4 6.0))
  (if (Variables|Default|GetStartCheck)
    (switch Utilities|FlowControl|Switch|SwitchonE_QuestionType (Variables|Default|GetQuestion%20Type)
      (:NewEnumerator0
        (Transformation|SetActorLocation _vector_3_4 (Transformation|GetActorLocation (Variables|Default|GetVector%201)) false false)
        (Class|IVector|MoveVectorHead(Message) _vector_3_4 (Variables|/Game/_PRACTICE/BP_VectorAnswer_NEW.BP_VectorAnswer_NEW_C|GetVector%20Head%20Loc (Variables|Default|GetVector%202)))
        (if (Utilities|CheckPosition (Variables|/Game/_PRACTICE/BP_VectorAnswer_NEW.BP_VectorAnswer_NEW_C|GetVector%20Head%20Loc (Variables|Default|GetVector%201)) (Transformation|GetActorLocation (Variables|Default|GetVector%202)) 16.0) :!label _label
          (Rendering|SetVisibility _defaultsceneroot_2 true true :!label _label_2)
          (else
            (Rendering|SetVisibility _defaultsceneroot_2 false true :!label _label_3))))
      (:NewEnumerator1
        (Transformation|SetActorLocation _vector_3_3 (Transformation|GetActorLocation (Variables|Default|GetVector%201)) false false)
        (Class|IVector|MoveVectorHead(Message) _vector_3_3 (- (Transformation|GetActorLocation _vector_2) (Default|GetCartesianCoordinates _vector_2)))
        (goto _label))
      (:NewEnumerator2
        (Transformation|SetActorLocation _vector_3_2 (+ _returnvalue_2 _returnvalue_5) false false)
        (Class|IVector|MoveVectorHead(Message) _vector_3_2 (+ _returnvalue_2 (* (Default|GetCartesianCoordinates _vector_1_2) (Variables|Default|GetScalar)) _returnvalue_5)))
      (:NewEnumerator4
        (if (Utilities|CheckPosition (Transformation|GetActorLocation (Variables|Default|GetVector%201)) (Transformation|GetActorLocation (Variables|Default|GetVector%202)) 16.0)
          (Default|SetDotText _aswb_operation_selector (Utilities|Text|ToText(Float) (Math|Vector|DotProduct (/ (Default|GetCartesianCoordinates (Variables|Default|GetVector%201)) 12.0) (/ (Default|GetCartesianCoordinates (Variables|Default|GetVector%202)) 12.0)) "HalfToEven" false true 1 324 1 1))
          (else
            (Default|SetDotText _aswb_operation_selector "-"))))
      (:NewEnumerator3
        (Transformation|SetActorLocation _vector_3 _returnvalue false false)
        (Class|IVector|MoveVectorHead(Message) _vector_3 (+ _returnvalue (* (Math|Vector|CrossProduct (/ (Default|GetCartesianCoordinates (Variables|Default|GetVector%201)) 12.0) (* (/ (Default|GetCartesianCoordinates (Variables|Default|GetVector%202)) 12.0) -1.0)) 12.0)))
        (if (Utilities|CheckPosition (Transformation|GetActorLocation (Variables|Default|GetVector%201)) (Transformation|GetActorLocation (Variables|Default|GetVector%202)) 16.0)
          (goto _label_2)
          (else
            (goto _label_3)))))))

(event EventBeginPlay
  (bind _mode_selector (Variables|Default|GetMode%20Selector))
  (bind _returnvalue (UserInterface|GetUserWidgetObject _mode_selector))
  (bind _aswb_operation_selector (Utilities|Casting|CastToWB_OperationSelector _returnvalue))
  (EventDispatchers|BindEventtoDispatchAddition _aswb_operation_selector (delegate Custom|Change%20Operation))
  (EventDispatchers|BindEventtoDispatchSubtraction _aswb_operation_selector (delegate Custom|Change%20Operation))
  (EventDispatchers|BindEventtoDispatchScalar _aswb_operation_selector (delegate Custom|Change%20Operation))
  (EventDispatchers|BindEventtoDispatchDot _aswb_operation_selector (delegate Custom|Change%20Operation))
  (EventDispatchers|BindEventtoDispatchCross _aswb_operation_selector (delegate Custom|Change%20Operation))
  (EventDispatchers|BindEventtoDispatchRaise _aswb_operation_selector (delegate Custom|Modify%20Scalar))
  (EventDispatchers|BindEventtoDispatchLower _aswb_operation_selector (delegate Custom|Modify%20Scalar))
  (EventDispatchers|BindEventtoDispatchMainMenu _aswb_operation_selector (delegate Custom|Return%20to%20Main%20Menu))
  (CallFunction|SpawnVectors))

(fn ConstructionScript)

(fn HideSecondVector
  (Transformation|SetActorLocation (Variables|Default|GetVector%202) "0.000000,0.000000,-500.000000" false false))

(fn ShowSecondVector
  (Transformation|SetActorLocation (Variables|Default|GetVector%202) (+ (Transformation|GetActorLocation) "0.000000,0.000000,20.000000") false false))