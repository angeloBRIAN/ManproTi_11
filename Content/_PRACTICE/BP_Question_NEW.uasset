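; Vector-math question actor for practice, posing random addition or subtraction problems on a text render and using spawned vector-answer actors as the response.
; BeginPlay spawns and binds one answer actor, adding a second, random operands and text only for Addition and Subtraction.
; CheckAnswer handles only Addition, testing head-to-tail placement from the origin and broadcasting the result.
; CheckTwoVectors leaves its distance comparison unwired, and CheckAnswerOld holds older distance and direction checks.
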(event EventBeginPlay
  (bind _returnvalue (Transformation|GetActorTransform))
  (bind _textrender (Variables|Default|GetTextRender))
  (bind _returnvalue_2 (Game|SpawnActorfromClass "/Game/_PRACTICE/BP_VectorAnswer_NEW.BP_VectorAnswer_NEW_C" (Math|Transform|MakeTransform (.location _returnvalue) (.rotation _returnvalue) "1.000000,1.000000,1.000000") "Undefined" 0 "(R=1.000000,G=0.000000,B=0.000000,A=1.000000)" 4e+01 0))
  (bind _output_get (Variables|Default|SetAnswer%201 _returnvalue_2))
  (EventDispatchers|BindEventtoCheckAnswer _output_get (EventDispatchers|CreateEvent :!event CheckAnswer))
  (switch Utilities|FlowControl|Switch|SwitchonE_QuestionType (Variables|Default|GetQuestionType)
    (:NewEnumerator0
      _)
    (:NewEnumerator1
      _))
  (bind _returnvalue_3 (Game|SpawnActorfromClass "/Game/_PRACTICE/BP_VectorAnswer_NEW.BP_VectorAnswer_NEW_C" (Math|Transform|MakeTransform (+ (.location _returnvalue) "0.000000,0.000000,20.000000") (.rotation _returnvalue) "1.000000,1.000000,1.000000") "Undefined" 0 "(R=0.000000,G=1.000000,B=0.000000,A=1.000000)" 4e+01 0))
  (bind _output_get_2 (Variables|Default|SetAnswer%202 _returnvalue_3))
  (EventDispatchers|BindEventtoCheckAnswer _output_get_2 (EventDispatchers|CreateEvent :!event CheckAnswer))
  (switch Utilities|FlowControl|Switch|SwitchonE_QuestionType (Variables|Default|GetQuestionType)
    (:NewEnumerator0
      _)
    (:NewEnumerator1
      _))
  (Variables|Default|SetQVector%201 (Math|Vector|MakeVector (Math|Random|RandomFloatinRange 0.0 5.0) (Math|Random|RandomFloatinRange 0.0 5.0) (Math|Random|RandomFloatinRange 0.0 5.0)))
  (Variables|Default|SetQVector%202 (Math|Vector|MakeVector (Math|Random|RandomFloatinRange 0.0 5.0) (Math|Random|RandomFloatinRange 0.0 5.0) (Math|Random|RandomFloatinRange 0.0 5.0)))
  (switch Utilities|FlowControl|Switch|SwitchonE_QuestionType (Variables|Default|GetQuestionType)
    (:NewEnumerator0
      (Rendering|Components|TextRender|SetText _textrender (Utilities|Text|FormatText "({0}, {1}, {2}) + ({3}, {4}, {5}) = ..." (.x (Variables|Default|GetQVector%201)) (.y (Variables|Default|GetQVector%201)) (.z (Variables|Default|GetQVector%201)) (.x (Variables|Default|GetQVector%202)) (.y (Variables|Default|GetQVector%202)) (.z (Variables|Default|GetQVector%202)))))
    (:NewEnumerator1
      (Rendering|Components|TextRender|SetText _textrender (Utilities|Text|FormatText "({0}, {1}, {2}) - ({3}, {4}, {5}) = ..." (.x (Variables|Default|GetQVector%201)) (.y (Variables|Default|GetQVector%201)) (.z (Variables|Default|GetQVector%201)) (.x (Variables|Default|GetQVector%202)) (.y (Variables|Default|GetQVector%202)) (.z (Variables|Default|GetQVector%202)))))
    (:NewEnumerator2
      (Rendering|Components|TextRender|SetText _textrender (Utilities|Text|FormatText "({0}, {1}, {2})" (.x (Variables|Default|GetQVector%201)) (.y (Variables|Default|GetQVector%201)) (.z (Variables|Default|GetQVector%201)))))
    (:NewEnumerator4
      (Rendering|Components|TextRender|SetText _textrender (Utilities|Text|FormatText "... . ... = ({0}, {1}, {2})" 0)))
    (:NewEnumerator3
      (Rendering|Components|TextRender|SetText _textrender (Utilities|Text|FormatText "({0}, {1}, {2}) x ({3}, {4}, {5}) = ..." (.x (Variables|Default|GetQVector%201)) (.y (Variables|Default|GetQVector%201)) (.z (Variables|Default|GetQVector%201)) (.x (Variables|Default|GetQVector%202)) (.y (Variables|Default|GetQVector%202)) (.z (Variables|Default|GetQVector%202)))))))

(fn ConstructionScript)

(fn CheckAnswerOld
  (params (Answer%20Vector%20End :type Vector))
  (bind _vectoranswer (Variables|Default|GetVectorAnswer))
  (bind _vectoranswer_2 (Variables|Default|GetVectorAnswer))
  (bind _awd1 (Variables|Default|Getawd1))
  (bind _returnvalue (Class|KismetMathLibrary|VectorDistanceSquared Answer%20Vector%20End _vectoranswer_2))
  (bind _returnvalue_2 (Math|Vector|Normalize _vectoranswer))
  (bind _returnvalue_3 (Transformation|GetActorLocation _awd1))
  (bind _returnvalue_4 (- Answer%20Vector%20End _returnvalue_3))
  (bind _returnvalue_5 (Math|Vector|Normalize _returnvalue_4))
  (bind _returnvalue_6 (Math|Vector|DotProduct _returnvalue_5 _returnvalue_2))
  (switch Utilities|FlowControl|Switch|SwitchonE_QuestionType (Variables|Default|GetQuestionType)
    (:NewEnumerator0
      (Development|PrintString (Utilities|String|ToString(Float) _returnvalue) :!label _label)
      (if (< _returnvalue 5e+01)
        (Utilities|FlowControl|DoOnce false :!label _label_2
          (:Completed
            (Default|CallCheckAnswerDispatch true)))))
    (:NewEnumerator1
      (goto _label))
    (:NewEnumerator2
      (goto _label))
    (:NewEnumerator3
      (Development|PrintString (Utilities|String|ToString(Float) _returnvalue_6))
      (if (> _returnvalue_6 0.9)
        (goto _label_2)))))

(fn RemoveSelf
  (Actor|DestroyActor (Variables|Default|GetAnswer%201)))

(fn CheckAnswer
  (bind _answer_1 (Variables|Default|GetAnswer%201))
  (bind _answer_2 (Variables|Default|GetAnswer%202))
  (bind _qvector_1 (Variables|Default|GetQVector%201))
  (bind _qvector_2 (Variables|Default|GetQVector%202))
  (bind _head_loc (Default|GetCartesianCoordinates _answer_2))
  (bind _head_loc_2 (Default|GetCartesianCoordinates _answer_1))
  (bind _returnvalue (Transformation|GetActorLocation _answer_1))
  (bind _returnvalue_2 (Transformation|GetActorLocation _answer_2))
  (bind _returnvalue_3 (Utilities|CheckTwoVectors _returnvalue_2 _head_loc_2 0.0))
  (bind _returnvalue_4 (Utilities|CheckTwoVectors :V1 _returnvalue :Tolerance 16.0))
  (bind _returnvalue_5 (Utilities|CheckTwoVectors _head_loc _qvector_2 16.0))
  (bind _returnvalue_6 (Utilities|CheckTwoVectors _head_loc_2 _qvector_1 16.0))
  (bind _returnvalue_7 (Math|Boolean|ANDBoolean _returnvalue_6 _returnvalue_4 _returnvalue_5 _returnvalue_3))
  (switch Utilities|FlowControl|Switch|SwitchonE_QuestionType (Variables|Default|GetQuestionType)
    (:NewEnumerator0
      (Development|PrintString (Utilities|String|ToString(Boolean) _returnvalue_7))
      (Default|CallCheckAnswerDispatch _returnvalue_7))))