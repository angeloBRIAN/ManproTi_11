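; Practice-mode question manager actor that runs questions chosen by type (addition, subtraction, scalar, dot, cross) from a question selector widget.
; Selector dispatchers replace the current BP_Question_NEW, whose answer dispatch drives timed status text.
; Correct answers spawn another question of the same type after a delay; wrong ones allow retrying.
; Main-menu requests remove the question, animate selector opacity, show the GI_NEW menu and destroy the manager.
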(event Custom|Respawn%20Question
  (params (Is%20Correct :type Boolean))
  (bind _question_selector (Variables|Default|GetQuestion%20Selector))
  (bind _returnvalue (UserInterface|GetUserWidgetObject _question_selector))
  (bind _aswb_question_selector (Utilities|Casting|CastToWB_QuestionSelector _returnvalue))
  (bind _statustext (Variables|/Game/_PRACTICE/WB_QuestionSelector.WB_QuestionSelector_C|GetstatusText _aswb_question_selector))
  (if Is%20Correct
    (bind _returnvalue_2 (Utilities|Time|SetTimerbyEvent (delegate Custom|TriggerRQ) 3.0))
    (Rendering|Components|TextRender|SetText _statustext "Correct! Next question in 3 seconds.")
    (Appearance|SetColorandOpacity _statustext (Utilities|Struct|MakeSlateColor "(R=0.250000,G=1.000000,B=0.250000,A=1.000000)") :!class /Script/UMG.TextBlock)
    (else
      (bind _returnvalue_3 (Utilities|Time|SetTimerbyEvent (delegate Custom|Remove%20False%20Text) 3.0))
      (Rendering|Components|TextRender|SetText _statustext "Incorrect! Try again.")
      (Appearance|SetColorandOpacity _statustext (Utilities|Struct|MakeSlateColor "(R=1.000000,G=0.050000,B=0.050000,A=1.000000)") :!class /Script/UMG.TextBlock))))

(event Custom|Remove%20False%20Text
  (Utilities|Time|ClearandInvalidateTimerbyHandle (stale Custom|Respawn%20Question _returnvalue_3))
  (Rendering|Components|TextRender|SetText (Variables|/Game/_PRACTICE/WB_QuestionSelector.WB_QuestionSelector_C|GetstatusText (.AsWB%20Question%20Selector (Utilities|Casting|CastToWB_QuestionSelector (UserInterface|GetUserWidgetObject (Variables|Default|GetQuestion%20Selector))))) ""))

(event Custom|Spawn%20Question
  (params (Question%20Type :type E_QuestionType%20Enum :default "NewEnumerator0"))
  (bind _returnvalue (Transformation|GetActorTransform))
  (Variables|Default|SetQuestion%20Type Question%20Type)
  (bind _returnvalue_2 (Game|SpawnActorfromClass "/Game/_PRACTICE/BP_Question_NEW.BP_Question_NEW_C" (Math|Transform|MakeTransform (.location _returnvalue) (.rotation _returnvalue) (.scale _returnvalue)) "Undefined" 0 (Variables|Default|GetQuestion%20Type) 0))
  (bind _output_get (Variables|Default|SetQuestion _returnvalue_2))
  (EventDispatchers|BindEventtoCheckAnswerDispatch _output_get (delegate Custom|Respawn%20Question)))

(event Custom|Return%20to%20Main%20Menu
  (bind _returnvalue (Game|GetGameInstance))
  (bind _question (Variables|Default|GetQuestion))
  (bind _asgi_new (Utilities|Casting|CastToGI_NEW _returnvalue))
  (bind _main_menu (Variables|/Game/_MAIN_MENU/GI_NEW.GI_NEW_C|GetMain%20Menu _asgi_new))
  (Default|RemoveSelf _question)
  (Actor|DestroyActor _question)
  (bind _awd (Timeline|timerShowMenu PlayFromStart)
    (:Update
      (Widget|SetRenderOpacity (UserInterface|GetUserWidgetObject (Variables|Default|GetQuestion%20Selector)) _awd))
    (:Finished
      (Widget|SetRenderOpacity (UserInterface|GetUserWidgetObject (Variables|/Game/_MAIN_MENU/BP_MainMenu.BP_MainMenu_C|GetMainMenuWidget _main_menu)) 1.0)
      (Default|ShowMainMenu _main_menu)
      (Actor|DestroyActor))))

(event Custom|reload%20question
  (params (Question%20Type :type E_QuestionType%20Enum :default "NewEnumerator0"))
  (bind _question (Variables|Default|GetQuestion))
  (Default|RemoveSelf _question)
  (Actor|DestroyActor _question)
  (CallFunction|SpawnQuestion Question%20Type))

(event Custom|TriggerRQ
  (bind _question (Variables|Default|GetQuestion))
  (Utilities|Time|ClearandInvalidateTimerbyHandle (stale Custom|Respawn%20Question _returnvalue_2))
  (Default|RemoveSelf _question)
  (Actor|DestroyActor _question)
  (CallFunction|SpawnQuestion (Variables|Default|GetQuestion%20Type))
  (Rendering|Components|TextRender|SetText (Variables|/Game/_PRACTICE/WB_QuestionSelector.WB_QuestionSelector_C|GetstatusText (.AsWB%20Question%20Selector (Utilities|Casting|CastToWB_QuestionSelector (UserInterface|GetUserWidgetObject (Variables|Default|GetQuestion%20Selector))))) ""))

(event EventBeginPlay
  (bind _question_selector (Variables|Default|GetQuestion%20Selector))
  (bind _returnvalue (UserInterface|GetUserWidgetObject _question_selector))
  (bind _aswb_question_selector (Utilities|Casting|CastToWB_QuestionSelector _returnvalue))
  (EventDispatchers|BindEventtoDispatchAddition _aswb_question_selector (delegate Custom|reload%20question))
  (EventDispatchers|BindEventtoDispatchSubtraction _aswb_question_selector (delegate Custom|reload%20question))
  (EventDispatchers|BindEventtoDispatchScalar _aswb_question_selector (delegate Custom|reload%20question))
  (EventDispatchers|BindEventtoDispatchDot _aswb_question_selector (delegate Custom|reload%20question))
  (EventDispatchers|BindEventtoDispatchCross _aswb_question_selector (delegate Custom|reload%20question))
  (EventDispatchers|BindEventtoDispatchMainMenu _aswb_question_selector (delegate Custom|Return%20to%20Main%20Menu)))

(fn ConstructionScript)