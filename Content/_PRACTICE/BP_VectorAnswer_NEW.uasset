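; Interactive 3D answer vector for a practice exercise, drawn as a colored arrow with a text label showing its name and components.
; MoveVectorHead stretches the arrow to a finger position, moves the sphere there and aims the actor using yaw and elevation axis-angle rotations.
; Tick derives Cartesian components from length and rotation, updating the head location and length-scaled label.
; Grab attaches it; release detaches it and fires CheckAnswer.
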(event EventBeginPlay
  (bind _vector (Variables|Default|GetVector))
  (Variables|/Script/Engine.ArrowComponent|SetArrowLength _vector (Variables|Default|GetVector%20Length))
  (Components|Arrow|SetArrowColor(LinearColor) _vector (Variables|Default|GetVector%20Color)))

(event EventReleaseVector
  (Transformation|DetachFromActor "KeepWorld" "KeepWorld" "KeepRelative")
  (Default|CallCheckAnswer))

(event EventTick
  (params (DeltaSeconds :type Float%20%28single-precision%29))
  (bind _head_loc (CallFunction|GetCartesianCoordinates))
  (bind _textrender (Variables|Default|GetTextRender))
  (bind (_x _y _z) (Utilities|OneDecimalVector _head_loc))
  (Variables|Default|SetVector%20Head%20Loc (+ (Transformation|GetActorLocation) (CallFunction|GetCartesianCoordinates)))
  (Rendering|Components|TextRender|SetText _textrender (Utilities|Text|FormatText "{0} ({1}, {2}, {3})" (Variables|Default|GetVector%20Name) _x _y _z))
  (Rendering|Components|TextRender|SetWorldSize _textrender (Math|Float|MapRangeClamped (Variables|/Script/Engine.ArrowComponent|GetArrowLength (Variables|Default|GetVector)) 6e+01 1.2e+02 18.0 3e+01)))

(event EventMoveVectorHead
  (params (Finger%20Pos :type Vector :default "0, 0, 0"))
  (CallFunction|MoveVectorHead Finger%20Pos))

(event EventGrabVector
  (params (Attach%20To :type Scene%20Component%20Object%20Reference))
  (Transformation|AttachComponentToComponent Attach%20To "None" "KeepWorld" "KeepWorld" "KeepRelative" true))

(fn ConstructionScript)

(fn MoveVectorHead
  (params (FingerPos :type Vector))
  (bind _returnvalue (Transformation|GetActorLocation))
  (bind _vector (Variables|Default|GetVector))
  (bind _returnvalue_2 (- FingerPos _returnvalue))
  (Variables|/Script/Engine.ArrowComponent|SetArrowLength _vector (Math|Vector|Distance(Vector) FingerPos _returnvalue))
  (Components|Arrow|SetArrowColor(LinearColor) _vector (Math|Conversions|ToLinearColor(Color) (Variables|/Script/Engine.ArrowComponent|GetArrowColor _vector)))
  (Transformation|SetWorldLocation (Variables|Default|GetSphere) FingerPos false false)
  (bind _output_get (Variables|Default|SetAngle%20XY (Class|KismetMathLibrary|DegAtan2 (.y _returnvalue_2) (.x _returnvalue_2))))
  (Transformation|SetActorRotation (Math|Vector|RotatorfromAxisandAngle "0.000000,0.000000,1.000000" _output_get))
  (bind _output_get_2 (Variables|Default|SetAngle%20Z (Class|KismetMathLibrary|DegAtan2 (.z _returnvalue_2) (Class|KismetMathLibrary|Hypotenuse (.x _returnvalue_2) (.y _returnvalue_2)))))
  (Class|Actor|AddActorWorldRotation (Math|Vector|RotatorfromAxisandAngle (Math|Vector|Normalize (Math|Vector|MakeVector (.y _returnvalue_2) (* (.x _returnvalue_2) -1.0) 0.0)) _output_get_2))
  (Variables|Default|SetIsVectorMoved true))

(fn GetCartesianCoordinates
  (return (Math|Vector|RotateVector (Math|Vector|MakeVector (Variables|/Script/Engine.ArrowComponent|GetArrowLength (Variables|Default|GetVector)) 0.0 0.0) (Transformation|GetActorRotation))))