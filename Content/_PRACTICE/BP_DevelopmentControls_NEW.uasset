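; Keyboard-driven development actor for testing grab and pinch interactions on vector objects.
; WASD/Space/Shift and numpad/Enter keys nudge Cube and Sphere in fixed world-space steps.
; Q toggles grabbing an overlapped I_Vector actor or releasing it; grab can instead trigger an I_Start actor.
; NumPad 7 toggles pinching, which shares AttachedObject with grab and sends Scene1's location each Tick to move the vector head.
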(event EventBeginPlay)

(event Collision|EventActorBeginOverlap
  (params (OtherActor :type Actor%20Object%20Reference)))

(event EventTick
  (params (DeltaSeconds :type Float%20%28single-precision%29))
  (if (Variables|Default|GetPinched)
    (CallFunction|MoveVectorHeadd)))

(event Input|KeyboardEvents|NumPadFour
  (params (Key :type Key%20Structure :default "None"))
  (:Pressed
    (Transformation|AddWorldOffset (Variables|Default|GetSphere) "0.000000,-10.000000,0.000000" false false)))

(event Input|KeyboardEvents|NumPadSix
  (params (Key :type Key%20Structure :default "None"))
  (:Pressed
    (Transformation|AddWorldOffset (Variables|Default|GetSphere) "0.000000,10.000000,0.000000" false false)))

(event Input|KeyboardEvents|Enter
  (params (Key :type Key%20Structure :default "None"))
  (:Pressed
    (Transformation|AddWorldOffset (Variables|Default|GetSphere) "0.000000,0.000000,-10.000000" false false)))

(event Input|KeyboardEvents|NumPadZero
  (params (Key :type Key%20Structure :default "None"))
  (:Pressed
    (Transformation|AddWorldOffset (Variables|Default|GetSphere) "0.000000,0.000000,10.000000" false false)))

(event Input|KeyboardEvents|Q
  (params (Key :type Key%20Structure :default "None"))
  (:Pressed
    (Utilities|FlowControl|FlipFlop
      (:A
        (CallFunction|Grab))
      (:B
        (CallFunction|Release)))))

(event Input|KeyboardEvents|NumPadSeven
  (params (Key :type Key%20Structure :default "None"))
  (:Pressed
    (Variables|Default|SetPinched (not (Variables|Default|GetPinched)))
    (Utilities|FlowControl|FlipFlop
      (:A
        (CallFunction|Pinch))
      (:B
        (Variables|Default|SetAttached%20Object 0)))))

(event Input|KeyboardEvents|W
  (params (Key :type Key%20Structure :default "None"))
  (:Pressed
    (Transformation|AddWorldOffset (Variables|Default|GetCube) "10.000000,0.000000,0.000000" false false)))

(event Input|KeyboardEvents|A
  (params (Key :type Key%20Structure :default "None"))
  (:Pressed
    (Transformation|AddWorldOffset (Variables|Default|GetCube) "0.000000,-10.000000,0.000000" false false)))

(event Input|KeyboardEvents|S
  (params (Key :type Key%20Structure :default "None"))
  (:Pressed
    (Transformation|AddWorldOffset (Variables|Default|GetCube) "-10.000000,0.000000,0.000000" false false)))

(event Input|KeyboardEvents|D
  (params (Key :type Key%20Structure :default "None"))
  (:Pressed
    (Transformation|AddWorldOffset (Variables|Default|GetCube) "0.000000,10.000000,0.000000" false false)))

(event Input|KeyboardEvents|LeftShift
  (params (Key :type Key%20Structure :default "None"))
  (:Pressed
    (Transformation|AddWorldOffset (Variables|Default|GetCube) "0.000000,0.000000,-10.000000" false false)))

(event Input|KeyboardEvents|SpaceBar
  (params (Key :type Key%20Structure :default "None"))
  (:Pressed
    (Transformation|AddWorldOffset (Variables|Default|GetCube) "0.000000,0.000000,10.000000" false false)))

(event Input|KeyboardEvents|NumPadEight
  (params (Key :type Key%20Structure :default "None"))
  (:Pressed
    (Transformation|AddWorldOffset (Variables|Default|GetSphere) "10.000000,0.000000,0.000000" false false)))

(event Input|KeyboardEvents|NumPadFive
  (params (Key :type Key%20Structure :default "None"))
  (:Pressed
    (Transformation|AddWorldOffset (Variables|Default|GetSphere) "-10.000000,0.000000,0.000000" false false)))

(fn ConstructionScript)

(fn Grab
  (bind _array_element (Utilities|Array|ForEachLoopwithBreak (Collision|GetOverlappingActors (Variables|Default|GetSphereC) 0 :!class /Script/Engine.PrimitiveComponent) :!label _label)
    (:LoopBody
      (Development|PrintString (Utilities|GetDisplayName _array_element))
      (if (Utilities|DoesObjectImplementInterface _array_element "/Game/_PRACTICE/I_Vector.I_Vector_C")
        (bind _output_get (Variables|Default|SetAttached%20Object _array_element))
        (Class|IVector|GrabVector(Message) _output_get (Variables|Default|GetScene))
        (goto _label Break)
        (elif (Utilities|DoesObjectImplementInterface _array_element "/Game/_PRACTICE/I_Start.I_Start_C")
          (Class|IStart|StartProgram(Message) _array_element)
          (goto _label Break))))))

(fn Release
  (bind _attached_object (Variables|Default|GetAttached%20Object)
    (:then
      (if (== (Transformation|GetAttachParent (Variables|/Script/Engine.Actor|GetRootComponent _attached_object)) (Variables|Default|GetSphereC))
        (Class|IVector|ReleaseVector(Message) _attached_object)
        (Variables|Default|SetAttached%20Object 0)))
    (:else)))

(fn Pinch
  (bind _array_element (Utilities|Array|ForEachLoopwithBreak (Collision|GetOverlappingActors (Variables|Default|GetSphereC1) 0 :!class /Script/Engine.PrimitiveComponent) :!label _label)
    (:LoopBody
      (Development|PrintString (Utilities|GetDisplayName _array_element))
      (if (Utilities|DoesObjectImplementInterface _array_element "/Game/_PRACTICE/I_Vector.I_Vector_C")
        (Variables|Default|SetAttached%20Object _array_element)
        (goto _label Break)))))

(fn Unpinch
  (Variables|Default|SetAttachedObjectR 0))

(fn MoveVectorHeadd
  (bind _attached_object (Variables|Default|GetAttached%20Object)
    (:then
      (Class|IVector|MoveVectorHead(Message) _attached_object (Transformation|GetWorldLocation (Variables|Default|GetScene1))))
    (:else)))