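; BP_LearnC1 is an animated tutorial display illustrating direction and magnitude with arrows, text labels and two divider cubes.
; On BeginPlay it plays the AnimationLoop timeline, whose tracks drive every animated element on each update.
; The tracks set one direction arrow's length and two magnitude arrows' lengths, resize both labels, and move the cubes vertically in unison.
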(event EventBeginPlay
  (bind (_direction _directionlength _dtextsize _magnitudelength _mtextsize _divisorpos) (Timeline|AnimationLoop PlayFromStart)
    (:Update
      (CallFunction|SetArrowLength (Variables|Default|GetArrow) _directionlength)
      (Rendering|Components|TextRender|SetWorldSize (Variables|Default|GetDirectionText) _dtextsize)
      (CallFunction|SetArrowLength (Variables|Default|GetArrow1) _magnitudelength)
      (CallFunction|SetArrowLength (Variables|Default|GetArrow2) _magnitudelength)
      (Rendering|Components|TextRender|SetWorldSize (Variables|Default|GetMagnitudeText) _mtextsize)
      (Transformation|SetRelativeLocation (Variables|Default|GetCube) (Math|Vector|MakeVector -0.25 0.0 _divisorpos) false false)
      (Transformation|SetRelativeLocation (Variables|Default|GetCube1) (Math|Vector|MakeVector 80.25 0.0 _divisorpos) false false))))

(fn ConstructionScript)