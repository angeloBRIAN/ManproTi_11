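; BP_hand is a VR hand actor that pairs a MotionController with an OculusXRHand component for one side, chosen by its Hand variable.
; The Construction Script turns Hand's enum name into the controller's motion source and sets the Oculus mesh and skeleton types through GetOculusHand.
; GetOculusHand maps Left and Right to their Oculus hand types and every other value to None.
; The event graph holds no active logic.
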(event EventBeginPlay)

(event Collision|EventActorBeginOverlap
  (params (OtherActor :type Actor%20Object%20Reference)))

(event EventTick
  (params (DeltaSeconds :type Float%20%28single-precision%29)))

(fn ConstructionScript
  (bind _returnvalue (CallFunction|GetOculusHand))
  (bind _oculusxrhand (Variables|Default|GetOculusXRHand))
  (Variables|/Script/HeadMountedDisplay.MotionControllerComponent|SetMotionSource (Variables|Default|GetMotionController) (Utilities|Name|EnumtoName (Variables|Default|Gethand)))
  (Variables|/Script/OculusXRInput.OculusXRHandComponent|SetMeshType _oculusxrhand _returnvalue)
  (Variables|/Script/OculusXRInput.OculusXRHandComponent|SetSkeletonType _oculusxrhand _returnvalue))

(fn GetOculusHand
  (return (Utilities|Select :Index (Variables|Default|Gethand) :Left "HandLeft" :Right "HandRight" :AnyHand "None" :Pad "None" :ExternalCamera "None" :Gun "None" :HMD "None" :Special_1 "None" :Special_2 "None" :Special_3 "None" :Special_4 "None" :Special_5 "None" :Special_6 "None" :Special_7 "None" :Special_8 "None" :Special_9 "None" :Special_10 "None" :Special_11 "None")))