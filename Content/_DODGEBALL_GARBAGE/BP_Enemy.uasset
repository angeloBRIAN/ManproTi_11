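; Dodgeball enemy that fires BP_Ball projectiles from its ShootDir component through three custom shot events, none triggered within this graph.
; ShootPlayer fires along the enemy's facing, and ShootPlayerMiss offsets that yaw for an intentional miss.
; ShootPlayerPredict leads the player, aiming above their location plus velocity times estimated travel time (distance over BulletSpeed).
; Each shot multiplies the spawned ball's ProjectileMovement velocity by BulletSpeed.
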(event Custom|ShootPlayerPredict
  (bind _returnvalue (Game|GetPlayerCharacter 0))
  (Utilities|IsValid _returnvalue
    (:Is%20Valid
      (bind _returnvalue_2 (Game|SpawnActorfromClass "/Game/AI/BP_Ball.BP_Ball_C" (Math|Transform|MakeTransform (Transformation|GetWorldLocation (Variables|Default|GetShootDir)) (Math|Rotator|FindLookatRotation (Transformation|GetWorldLocation (Variables|Default|GetShootDir)) (+ (+ (Transformation|GetActorLocation _returnvalue) "0.000000,0.000000,80.000000") (* (Transformation|GetVelocity _returnvalue) (/ (Transformation|GetDistanceTo _returnvalue) (Variables|Default|GetBulletSpeed))))) "1.000000,1.000000,1.000000") "Undefined" 0 0))
      (Variables|/Script/Engine.MovementComponent|SetVelocity (Variables|/Game/AI/BP_Ball.BP_Ball_C|GetProjectileMovement _returnvalue_2) (* (Variables|/Script/Engine.MovementComponent|GetVelocity (Variables|/Game/AI/BP_Ball.BP_Ball_C|GetProjectileMovement _returnvalue_2)) (Variables|Default|GetBulletSpeed))))))

(event Custom|ShootPlayerMiss
  (bind _returnvalue (Transformation|GetActorRotation))
  (bind _returnvalue_2 (Game|SpawnActorfromClass "/Game/AI/BP_Ball.BP_Ball_C" (Math|Transform|MakeTransform (Transformation|GetWorldLocation (Variables|Default|GetShootDir)) (Math|Rotator|MakeRotator (.roll _returnvalue) (.pitch _returnvalue) (+ (.yaw _returnvalue) 3e+01))) "Undefined" 0 0))
  (Variables|/Script/Engine.MovementComponent|SetVelocity (Variables|/Game/AI/BP_Ball.BP_Ball_C|GetProjectileMovement _returnvalue_2) (* (Variables|/Script/Engine.MovementComponent|GetVelocity (Variables|/Game/AI/BP_Ball.BP_Ball_C|GetProjectileMovement _returnvalue_2)) (Variables|Default|GetBulletSpeed))))

(event Custom|ShootPlayer
  (bind _returnvalue (Game|SpawnActorfromClass "/Game/AI/BP_Ball.BP_Ball_C" (Math|Transform|MakeTransform (Transformation|GetWorldLocation (Variables|Default|GetShootDir)) (Transformation|GetActorRotation)) "Undefined" 0 0))
  (Variables|/Script/Engine.MovementComponent|SetVelocity (Variables|/Game/AI/BP_Ball.BP_Ball_C|GetProjectileMovement _returnvalue) (* (Variables|/Script/Engine.MovementComponent|GetVelocity (Variables|/Game/AI/BP_Ball.BP_Ball_C|GetProjectileMovement _returnvalue)) (Variables|Default|GetBulletSpeed))))

(event Collision|EventActorBeginOverlap
  (params (OtherActor :type Actor%20Object%20Reference)))

(fn ConstructionScript)