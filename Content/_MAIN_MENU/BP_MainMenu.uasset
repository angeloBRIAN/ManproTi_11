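; Main menu actor hosting a widget component whose Tutorial, Freemode and Practice dispatchers launch each mode.
; Timelines animate the actor's height for Practice and Freemode or fade widget opacity for Tutorial, then spawn that mode's actor and hide the menu.
; Practice and Freemode also build a shared 3D grid of BP_GridSegment actors, trimming cube components on upper edges, plus a BP_GridZero.
; ShowMainMenu restores widget visibility and the actor's position.
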(event Custom|Tutorial
  (bind _returnvalue (Transformation|GetActorTransform))
  (bind _fade (Timeline|TutorialFade PlayFromStart)
    (:Update
      (Widget|SetRenderOpacity (UserInterface|GetUserWidgetObject (Variables|Default|GetMainMenuWidget)) _fade))
    (:Finished
      (Game|SpawnActorfromClass "/Game/UI/BP_OpsiMateri.BP_OpsiMateri_C" (Math|Transform|MakeTransform (Math|Vector|MakeVector (.x (.location _returnvalue)) (.y (.location _returnvalue)) 45.0) (.rotation _returnvalue) (.scale _returnvalue)) "Undefined" 0 0)
      (CallFunction|HideMainMenu))))

(event Custom|Practice
  (bind _returnvalue (Transformation|GetActorTransform))
  (bind _fade (Timeline|Timeline PlayFromStart)
    (:Update
      (Transformation|SetActorLocation (Math|Vector|MakeVector 8e+01 0.0 _fade) false false))
    (:Finished
      (Game|SpawnActorfromClass "/Game/_PRACTICE/BP_QuestionManager_NEW.BP_QuestionManager_NEW_C" (Math|Transform|MakeTransform (Math|Vector|MakeVector (.x (.location _returnvalue)) (.y (.location _returnvalue)) 45.0) (.rotation _returnvalue) (.scale _returnvalue)) "Undefined" 0 0)
      (CallFunction|HideMainMenu)
      (for _index (range -4 4)
        (for _index_2 (range -4 4)
          (for _index_3 (range -1 1)
            (bind _returnvalue_2 (Game|SpawnActorfromClass "/Game/_MAIN_MENU/BP_GridSegment.BP_GridSegment_C" (Math|Transform|MakeTransform (* (Math|Vector|MakeVector (Math|Conversions|ToFloat(Integer) _index) (Math|Conversions|ToFloat(Integer) _index_2) (Math|Conversions|ToFloat(Integer) _index_3)) 6e+01) "0, 0, 0" "1.000000,1.000000,1.000000") "Undefined" 0 0))
            (Utilities|Array|Add (Variables|Default|GetGrids) _returnvalue_2)
            (if (== _index 4)
              (Default|RemoveComponent _returnvalue_2 (Variables|/Game/_MAIN_MENU/BP_GridSegment.BP_GridSegment_C|GetCube1 _returnvalue_2)))
            (if (== _index_2 4)
              (Default|RemoveComponent _returnvalue_2 (Variables|/Game/_MAIN_MENU/BP_GridSegment.BP_GridSegment_C|GetCube2 _returnvalue_2)))
            (if (== _index_3 1)
              (Default|RemoveComponent _returnvalue_2 (Variables|/Game/_MAIN_MENU/BP_GridSegment.BP_GridSegment_C|GetCube _returnvalue_2))))))
      (bind _returnvalue_3 (Game|SpawnActorfromClass "/Game/_MAIN_MENU/BP_GridZero.BP_GridZero_C" (Math|Transform|MakeTransform "0, 0, 0" "0, 0, 0" "1.000000,1.000000,1.000000") "Undefined" 0 0))
      (Variables|Default|SetGridZero _returnvalue_3))))

(event Custom|Freemode
  (bind _returnvalue (Transformation|GetActorTransform))
  (bind _fade (Timeline|Timeline_0 PlayFromStart)
    (:Update
      (Transformation|SetActorLocation (Math|Vector|MakeVector 8e+01 0.0 _fade) false false))
    (:Finished
      (Game|SpawnActorfromClass "/Game/_PRACTICE/BP_FreemodeManager.BP_FreemodeManager_C" (Math|Transform|MakeTransform (Math|Vector|MakeVector (.x (.location _returnvalue)) (.y (.location _returnvalue)) 45.0) (.rotation _returnvalue) (.scale _returnvalue)) "Undefined" 0 0)
      (CallFunction|HideMainMenu)
      (for _index (range -4 4)
        (for _index_2 (range -4 4)
          (for _index_3 (range -1 1)
            (bind _returnvalue_2 (Game|SpawnActorfromClass "/Game/_MAIN_MENU/BP_GridSegment.BP_GridSegment_C" (Math|Transform|MakeTransform (* (Math|Vector|MakeVector (Math|Conversions|ToFloat(Integer) _index) (Math|Conversions|ToFloat(Integer) _index_2) (Math|Conversions|ToFloat(Integer) _index_3)) 6e+01) "0, 0, 0" "1.000000,1.000000,1.000000") "Undefined" 0 0))
            (Utilities|Array|Add (Variables|Default|GetGrids) _returnvalue_2)
            (if (== _index 4)
              (Default|RemoveComponent _returnvalue_2 (Variables|/Game/_MAIN_MENU/BP_GridSegment.BP_GridSegment_C|GetCube1 _returnvalue_2)))
            (if (== _index_2 4)
              (Default|RemoveComponent _returnvalue_2 (Variables|/Game/_MAIN_MENU/BP_GridSegment.BP_GridSegment_C|GetCube2 _returnvalue_2)))
            (if (== _index_3 1)
              (Default|RemoveComponent _returnvalue_2 (Variables|/Game/_MAIN_MENU/BP_GridSegment.BP_GridSegment_C|GetCube _returnvalue_2))))))
      (bind _returnvalue_3 (Game|SpawnActorfromClass "/Game/_MAIN_MENU/BP_GridZero.BP_GridZero_C" (Math|Transform|MakeTransform "0, 0, 0" "0, 0, 0" "1.000000,1.000000,1.000000") "Undefined" 0 0))
      (Variables|Default|SetGridZero _returnvalue_3))))

(event EventBeginPlay
  (bind _mainmenuwidget (Variables|Default|GetMainMenuWidget))
  (bind _returnvalue (UserInterface|GetUserWidgetObject _mainmenuwidget))
  (bind _aswb_main_menu_new (Utilities|Casting|CastToWB_MainMenu_NEW _returnvalue))
  (EventDispatchers|BindEventtoTutorialDispatch _aswb_main_menu_new (delegate Custom|Tutorial))
  (EventDispatchers|BindEventtoFreemodeDispatch _aswb_main_menu_new (delegate Custom|Freemode))
  (EventDispatchers|BindEventtoPracticeDispatch _aswb_main_menu_new (delegate Custom|Practice)))

(fn ConstructionScript)

(fn HideMainMenu
  (Rendering|SetVisibility (Variables|Default|GetMainMenuWidget) false false))

(fn ShowMainMenu
  (Rendering|SetVisibility (Variables|Default|GetMainMenuWidget) true false)
  (Transformation|SetActorLocation "80.000000,0.000000,45.000000" false false))