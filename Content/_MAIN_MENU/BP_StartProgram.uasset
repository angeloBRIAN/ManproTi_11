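; Startup actor that plays the main menu intro, triggered one second after BeginPlay or directly through StartProgram.
; It spawns BP_MainMenu at an offset, stores it in GI_NEW and removes its own text render.
; A timeline scales and rotates its cube while fading in the menu widget.
; When finished, nested loops build a world-origin lattice of BP_GridSegment actors, trimming components on the upper edges, then the actor destroys itself.
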(event EventStartProgram
  (bind _returnvalue (Transformation|GetActorTransform))
  (bind _cube (Variables|Default|GetCube))
  (bind _returnvalue_2 (Game|SpawnActorfromClass "/Game/_MAIN_MENU/BP_MainMenu.BP_MainMenu_C" (Math|Transform|MakeTransform (+ (.location _returnvalue) "60.000000,0.000000,60.000000") (.rotation _returnvalue) "1.000000,1.000000,1.000000") "Undefined" 0 0))
  (Variables|/Game/_MAIN_MENU/GI_NEW.GI_NEW_C|SetMain%20Menu (.AsGI%20NEW (Utilities|Casting|CastToGI_NEW (Game|GetGameInstance))) _returnvalue_2)
  (Components|DestroyComponent (Variables|Default|GetTextRender))
  (bind (_direction _scale _rotate _main_menu_visibility) (Timeline|Timeline PlayFromStart)
    (:Update
      (Transformation|SetRelativeScale3D _cube (Math|Vector|MakeVector _scale _scale _scale))
      (Transformation|SetRelativeRotation _cube (Math|Rotator|MakeRotator 0.0 0.0 _rotate) false false)
      (Widget|SetRenderOpacity (UserInterface|GetWidget (Variables|/Game/_MAIN_MENU/BP_MainMenu.BP_MainMenu_C|GetMainMenuWidget _returnvalue_2)) _main_menu_visibility))
    (:Finished
      (for _index (range -4 4)
        (for _index_2 (range -4 4)
          (for _index_3 (range -1 1)
            (bind _returnvalue_3 (Game|SpawnActorfromClass "/Game/_MAIN_MENU/BP_GridSegment.BP_GridSegment_C" (Math|Transform|MakeTransform (* (Math|Vector|MakeVector (Math|Conversions|ToFloat(Integer) _index) (Math|Conversions|ToFloat(Integer) _index_2) (Math|Conversions|ToFloat(Integer) _index_3)) 6e+01) "0, 0, 0" "1.000000,1.000000,1.000000") "Undefined" 0 0))
            (if (== _index 4)
              (Default|RemoveComponent _returnvalue_3 (Variables|/Game/_MAIN_MENU/BP_GridSegment.BP_GridSegment_C|GetCube1 _returnvalue_3)))
            (if (== _index_2 4)
              (Default|RemoveComponent _returnvalue_3 (Variables|/Game/_MAIN_MENU/BP_GridSegment.BP_GridSegment_C|GetCube2 _returnvalue_3)))
            (if (== _index_3 1)
              (Default|RemoveComponent _returnvalue_3 (Variables|/Game/_MAIN_MENU/BP_GridSegment.BP_GridSegment_C|GetCube _returnvalue_3))))))
      (Actor|DestroyActor))))

(event EventBeginPlay
  (bind _returnvalue (Transformation|GetActorTransform))
  (bind _cube (Variables|Default|GetCube))
  (Utilities|FlowControl|Delay 1.0)
  (bind _returnvalue_2 (Game|SpawnActorfromClass "/Game/_MAIN_MENU/BP_MainMenu.BP_MainMenu_C" (Math|Transform|MakeTransform (+ (.location _returnvalue) "60.000000,0.000000,60.000000") (.rotation _returnvalue) "1.000000,1.000000,1.000000") "Undefined" 0 0))
  (Variables|/Game/_MAIN_MENU/GI_NEW.GI_NEW_C|SetMain%20Menu (.AsGI%20NEW (Utilities|Casting|CastToGI_NEW (Game|GetGameInstance))) _returnvalue_2)
  (Components|DestroyComponent (Variables|Default|GetTextRender))
  (bind (_direction _scale _rotate _main_menu_visibility) (Timeline|Timeline PlayFromStart)
    (:Update
      (Transformation|SetRelativeScale3D _cube (Math|Vector|MakeVector _scale _scale _scale))
      (Transformation|SetRelativeRotation _cube (Math|Rotator|MakeRotator 0.0 0.0 _rotate) false false)
      (Widget|SetRenderOpacity (UserInterface|GetWidget (Variables|/Game/_MAIN_MENU/BP_MainMenu.BP_MainMenu_C|GetMainMenuWidget _returnvalue_2)) _main_menu_visibility))
    (:Finished
      (for _index (range -4 4)
        (for _index_2 (range -4 4)
          (for _index_3 (range -1 1)
            (bind _returnvalue_3 (Game|SpawnActorfromClass "/Game/_MAIN_MENU/BP_GridSegment.BP_GridSegment_C" (Math|Transform|MakeTransform (* (Math|Vector|MakeVector (Math|Conversions|ToFloat(Integer) _index) (Math|Conversions|ToFloat(Integer) _index_2) (Math|Conversions|ToFloat(Integer) _index_3)) 6e+01) "0, 0, 0" "1.000000,1.000000,1.000000") "Undefined" 0 0))
            (if (== _index 4)
              (Default|RemoveComponent _returnvalue_3 (Variables|/Game/_MAIN_MENU/BP_GridSegment.BP_GridSegment_C|GetCube1 _returnvalue_3)))
            (if (== _index_2 4)
              (Default|RemoveComponent _returnvalue_3 (Variables|/Game/_MAIN_MENU/BP_GridSegment.BP_GridSegment_C|GetCube2 _returnvalue_3)))
            (if (== _index_3 1)
              (Default|RemoveComponent _returnvalue_3 (Variables|/Game/_MAIN_MENU/BP_GridSegment.BP_GridSegment_C|GetCube _returnvalue_3))))))
      (Actor|DestroyActor))))

(fn ConstructionScript)