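; BP_VectorAxis is an actor showing an adjustable single-axis vector as an arrow with a sphere handle and text readout.
; MoveVectorHead projects a supplied finger position onto the selected X, Y or Z axis, moving the sphere, resizing the arrow and flagging the vector as moved.
; Tick writes arrow length to the display, leaving both degree fields unfed, and recomputes the head location from actor location, rotation and length.
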(event EventBeginPlay
  (bind _vectorarrow (Variables|Default|GetVectorArrow))
  (bind _output_get (Variables|/Script/Engine.ArrowComponent|SetArrowLength _vectorarrow (Variables|Default|GetVector%20Length)))
  (Components|Arrow|SetArrowColor(LinearColor) _vectorarrow (Variables|Default|GetVector%20Color)))

(event EventTick
  (params (DeltaSeconds :type Float%20%28single-precision%29))
  (Rendering|Components|TextRender|SetText (Variables|Default|GetDisplay) (Utilities|Text|FormatText "{0}, {1}°, {2}°" (Variables|/Script/Engine.ArrowComponent|GetArrowLength (Variables|Default|GetVectorArrow))))
  (Variables|Default|SetVector%20Head%20Loc (+ (Transformation|GetActorLocation) (Math|Vector|RotateVector (Math|Vector|MakeVector (stale EventBeginPlay _output_get) 0.0 0.0) (Transformation|GetActorRotation)))))

(fn ConstructionScript)

(fn MoveVectorHead
  (params (FingerPos :type Vector))
  (bind (_x _y _z) (Math|Vector|BreakVector FingerPos))
  (bind _returnvalue (Transformation|GetActorLocation))
  (bind _vectorarrow (Variables|Default|GetVectorArrow))
  (bind _sphere (Variables|Default|GetSphere))
  (bind _vectorarrow_2 (Variables|Default|GetVectorArrow))
  (bind _returnvalue_2 (- FingerPos _returnvalue))
  (bind (_x_2 _y_2 _z_2) (Math|Vector|BreakVector _returnvalue_2))
  (switch Utilities|FlowControl|Switch|SwitchonE_Axis (Variables|Default|GetAxis)
    (:NewEnumerator0
      (Variables|Default|SetVector%20Head%20Loc (Math|Vector|MakeVector _x 0.0 0.0))
      (Transformation|SetWorldLocation _sphere (Math|Vector|MakeVector _x 0.0 0.0) false false)
      (Variables|/Script/Engine.ArrowComponent|SetArrowLength _vectorarrow_2 _x_2))
    (:NewEnumerator1
      (Variables|Default|SetVector%20Head%20Loc (Math|Vector|MakeVector 0.0 _y 0.0))
      (Transformation|SetWorldLocation _sphere (Math|Vector|MakeVector 0.0 _y 0.0) false false)
      (Variables|/Script/Engine.ArrowComponent|SetArrowLength _vectorarrow_2 _y_2))
    (:NewEnumerator2
      (Variables|Default|SetVector%20Head%20Loc (Math|Vector|MakeVector 0.0 0.0 _z))
      (Transformation|SetWorldLocation _sphere (Math|Vector|MakeVector 0.0 0.0 _z) false false)
      (Variables|/Script/Engine.ArrowComponent|SetArrowLength _vectorarrow_2 _z_2)))
  (Components|Arrow|SetArrowColor(LinearColor) _vectorarrow (Math|Conversions|ToLinearColor(Color) (Variables|/Script/Engine.ArrowComponent|GetArrowColor _vectorarrow)))
  (Variables|Default|SetIsVectorMoved true))