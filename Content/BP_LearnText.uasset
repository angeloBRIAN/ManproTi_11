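; Slideshow tutorial actor that presents learning slides, each a title and description on a WB_TutorialDisplay widget plus a display actor spawned above it.
; BeginPlay spawns a hardcoded BP_VectorLearn1, fills text from row "NewRow" and binds the widget's previous, next and exit dispatchers.
; Slide functions step through DataTable rows, replacing the display and text and toggling arrow visibility.
; Exit spawns BP_OpsiMateri, then destroys the display and itself.
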(event Custom|exitToSelect
  (Game|SpawnActorfromClass "/Game/UI/BP_OpsiMateri.BP_OpsiMateri_C" (Transformation|GetActorTransform) "Undefined" 0 0)
  (Actor|DestroyActor (Variables|Default|GetCurrentDisplay))
  (Actor|DestroyActor))

(event EventBeginPlay
  (bind _widget (Variables|Default|GetWidget))
  (bind _returnvalue (UserInterface|GetUserWidgetObject _widget))
  (bind _aswb_tutorial_display (Utilities|Casting|CastToWB_TutorialDisplay _returnvalue))
  (bind _returnvalue_2 (Game|SpawnActorfromClass "/Game/_TUTORIAL_OLD/BP_VectorLearn1.BP_VectorLearn1_C" (Math|Transform|MakeTransform (+ (Transformation|GetActorLocation) "0.000000,0.000000,100.000000") "0, 0, 0" "1.000000,1.000000,1.000000") "Undefined" 0 0))
  (Variables|Default|SetCurrentDisplay _returnvalue_2)
  (bind _aswb_tutorial_display_2 (Utilities|Casting|CastToWB_TutorialDisplay (UserInterface|GetWidget (Variables|Default|GetWidget))))
  (EventDispatchers|BindEventtoPrevSlide _aswb_tutorial_display_2 (EventDispatchers|CreateEvent :!event PreviousSlide))
  (EventDispatchers|BindEventtoNextSlide _aswb_tutorial_display_2 (EventDispatchers|CreateEvent :!event NextSlide))
  (EventDispatchers|BindEventtoExitDispatch _aswb_tutorial_display_2 (delegate Custom|exitToSelect))
  (bind _returnvalue_3 (Utilities|GetDataTableRow (Variables|Default|GetDataTable) "NewRow")
    (:then
      (Rendering|Components|TextRender|SetText (Variables|/Game/_DODGEBALL_GARBAGE/WB_TutorialDisplay.WB_TutorialDisplay_C|GettitleText _aswb_tutorial_display) (.Title (Utilities|Struct|BreakS_LearnData _returnvalue_3)))
      (Rendering|Components|TextRender|SetText (Variables|/Game/_DODGEBALL_GARBAGE/WB_TutorialDisplay.WB_TutorialDisplay_C|GetdescText _aswb_tutorial_display) (.Description (Utilities|Struct|BreakS_LearnData _returnvalue_3))))))

(event Collision|EventActorBeginOverlap
  (params (OtherActor :type Actor%20Object%20Reference)))

(event EventTick
  (params (DeltaSeconds :type Float%20%28single-precision%29)))

(fn ConstructionScript)

(fn PreviousSlide
  (bind _datatable (Variables|Default|GetDataTable))
  (bind _widget (Variables|Default|GetWidget))
  (bind _returnvalue (UserInterface|GetUserWidgetObject _widget))
  (bind _aswb_tutorial_display (Utilities|Casting|CastToWB_TutorialDisplay _returnvalue))
  (if (> (Variables|Default|GetCurrentSlide) 0)
    (Math|Integer|DecrementInt (Variables|Default|GetCurrentSlide)
      (:%20%20
        (Actor|DestroyActor (Variables|Default|GetCurrentDisplay))
        (bind _outrownames (DataTable|GetDataTableRowNames _datatable))
        (bind _returnvalue_2 (Utilities|GetDataTableRow _datatable (Utilities|Array|Get(acopy) _outrownames (Variables|Default|GetCurrentSlide)))
          (:then
            (bind _returnvalue_3 (Game|SpawnActorfromClass (.DIsplay (Utilities|Struct|BreakS_LearnData _returnvalue_2)) (Math|Transform|MakeTransform (+ (Transformation|GetActorLocation) "0.000000,0.000000,100.000000") "0, 0, 0" "1.000000,1.000000,1.000000") "Undefined" 0 0))
            (Variables|Default|SetCurrentDisplay _returnvalue_3)
            (Rendering|Components|TextRender|SetText (Variables|/Game/_DODGEBALL_GARBAGE/WB_TutorialDisplay.WB_TutorialDisplay_C|GettitleText _aswb_tutorial_display) (.Title (Utilities|Struct|BreakS_LearnData _returnvalue_2)))
            (Rendering|Components|TextRender|SetText (Variables|/Game/_DODGEBALL_GARBAGE/WB_TutorialDisplay.WB_TutorialDisplay_C|GetdescText _aswb_tutorial_display) (.Description (Utilities|Struct|BreakS_LearnData _returnvalue_2)))
            (if (== (Variables|Default|GetCurrentSlide) 0)
              (Widget|SetVisibility (Variables|/Game/_DODGEBALL_GARBAGE/WB_TutorialDisplay.WB_TutorialDisplay_C|GetoverlayPrev _aswb_tutorial_display) "Hidden"))
            (bind _outrownames_2 (DataTable|GetDataTableRowNames (Variables|Default|GetDataTable)))
            (if (< (Variables|Default|GetCurrentSlide) (- (Utilities|Array|Length _outrownames_2) 1))
              (Widget|SetVisibility (Variables|/Game/_DODGEBALL_GARBAGE/WB_TutorialDisplay.WB_TutorialDisplay_C|GetoverlayNext _aswb_tutorial_display) "Visible"))))))
    (else
      (Variables|Default|SetCurrentSlide 0))))

(fn NextSlide
  (bind _datatable (Variables|Default|GetDataTable))
  (bind _widget (Variables|Default|GetWidget))
  (bind _returnvalue (UserInterface|GetUserWidgetObject _widget))
  (bind _aswb_tutorial_display (Utilities|Casting|CastToWB_TutorialDisplay _returnvalue))
  (bind _outrownames (DataTable|GetDataTableRowNames (Variables|Default|GetDataTable)))
  (if (< (Variables|Default|GetCurrentSlide) (- (Utilities|Array|Length _outrownames) 1))
    (Math|Integer|IncrementInt (Variables|Default|GetCurrentSlide)
      (:%20%20
        (Actor|DestroyActor (Variables|Default|GetCurrentDisplay))
        (bind _outrownames_2 (DataTable|GetDataTableRowNames _datatable))
        (bind _returnvalue_2 (Utilities|GetDataTableRow _datatable (Utilities|Array|Get(acopy) _outrownames_2 (Variables|Default|GetCurrentSlide)))
          (:then
            (bind _returnvalue_3 (Game|SpawnActorfromClass (.DIsplay (Utilities|Struct|BreakS_LearnData _returnvalue_2)) (Math|Transform|MakeTransform (+ (Transformation|GetActorLocation) "0.000000,0.000000,100.000000") "0, 0, 0" "1.000000,1.000000,1.000000") "Undefined" 0 0))
            (Variables|Default|SetCurrentDisplay _returnvalue_3)
            (Rendering|Components|TextRender|SetText (Variables|/Game/_DODGEBALL_GARBAGE/WB_TutorialDisplay.WB_TutorialDisplay_C|GettitleText _aswb_tutorial_display) (.Title (Utilities|Struct|BreakS_LearnData _returnvalue_2)))
            (Rendering|Components|TextRender|SetText (Variables|/Game/_DODGEBALL_GARBAGE/WB_TutorialDisplay.WB_TutorialDisplay_C|GetdescText _aswb_tutorial_display) (.Description (Utilities|Struct|BreakS_LearnData _returnvalue_2)))
            (if (> (Variables|Default|GetCurrentSlide) 0)
              (Widget|SetVisibility (Variables|/Game/_DODGEBALL_GARBAGE/WB_TutorialDisplay.WB_TutorialDisplay_C|GetoverlayPrev _aswb_tutorial_display) "Visible"))
            (bind _outrownames_3 (DataTable|GetDataTableRowNames (Variables|Default|GetDataTable)))
            (if (== (- (Utilities|Array|Length _outrownames_3) 1) (Variables|Default|GetCurrentSlide))
              (Widget|SetVisibility (Variables|/Game/_DODGEBALL_GARBAGE/WB_TutorialDisplay.WB_TutorialDisplay_C|GetoverlayNext _aswb_tutorial_display) "Hidden"))))))
    (else
      (Variables|Default|SetCurrentSlide (- (Utilities|Array|Length _outrownames) 1)))))